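; Arrow projectile for the Oni Archer enemy that deals damage through a hitbox message exchange.
; Each tick, a force along its forward vector propels the physics mesh while horizontal speed is below a cap.
; When another actor requests hitbox damage, it sends its arrow damage back to that actor.
; A lifetime timer or overlap with a Hero-tagged actor destroys it after a one-tick delay.
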(event OnComponentBeginOverlap(MEsh)
  (params (OverlappedComponent :type Primitive%20Component%20Object%20Reference) (OtherActor :type Actor%20Object%20Reference) (OtherComp :type Primitive%20Component%20Object%20Reference) (OtherBodyIndex :type Integer) (bFromSweep :type Boolean) (SweepResult :type Hit%20Result%20Structure%20%28by%20ref%29))
  (if (Actor|ActorHasTag OtherActor "Hero")
    (CallFunction|DestroyArrow)))

(event Custom|DestroyArrow
  (Utilities|FlowControl|DelayUntilNextTick)
  (Actor|DestroyActor))

(event EventGetHitboxDamage
  (params (ActorToDamage :type Actor%20Object%20Reference))
  (Class|BISendHitboxDamage|SendHitboxDamage(Message) ActorToDamage (Variables|Default|GetarrowDamage)))

(event EventTick
  (params (DeltaSeconds :type Float%20%28single-precision%29))
  (bind _returnvalue (Physics|GetPhysicsLinearVelocity (Variables|Character|GetMesh) "None"))
  (if (< (Math|Vector|VectorLengthXY _returnvalue) 1.3e+03)
    (Physics|AddForce (Variables|Character|GetMesh) (* (Transformation|GetActorForwardVector) (Variables|Default|GetarrowSpeed)) "None" false)))

(event EventBeginPlay
  (Utilities|Time|SetTimerbyEvent (delegate Custom|DestroyArrow) (Variables|Default|GetarrowLife)))

(fn ConstructionScript)