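; Oni brawler enemy that wanders the navmesh, targets reachable tagged heroes and fights them in melee.
; It holds at wait range, backing away when crowded, and requests aggro from its hero until permitted to close in.
; Timer-driven checks chain random hook, punch or headbutt attacks using delayed, temporary box hitboxes.
; Damage is exchanged by messages, driving hitstun and death, while sightings and Satoshi's grapple trigger retargeting.
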(event OnComponentBeginOverlap(HurtBox)
  (params (OverlappedComponent :type Primitive%20Component%20Object%20Reference) (OtherActor :type Actor%20Object%20Reference) (OtherComp :type Primitive%20Component%20Object%20Reference) (OtherBodyIndex :type Integer) (bFromSweep :type Boolean) (SweepResult :type Hit%20Result%20Structure%20%28by%20ref%29))
  ;[1 1 1 1 32] Take Damage
  (if (Components|ComponentHasTag OtherComp (Variables|Hitbox|GetHeroHitboxTagName)) ; If hurtbox was overlapped by hostile hitbox.
    (Variables|Default|SetlastOffendingActor OtherActor)
    (Class|BIGetHitboxDamage|GetHitboxDamage(Message) OtherActor self)
    (if (Actor|ActorHasTag "Hero")
      (Utilities|IsValid OtherActor ; Has not died
        (:Is%20Valid
          (CallFunction|ChangeHeroTarget)
          (Variables|Default|SetisWandering false))))))

(event Custom|ResetAttackState
  ;[1 1 1] After Attack
  (CallFunction|CheckAttackState))

(event Custom|ApplyHitstun
  ;[1 1 1] Hitstun
  (Variables|Default|SetinHitstun true)
  (Utilities|Time|ClearandInvalidateTimerbyHandle (stale _returnvalue))
  (bind _returnvalue (Utilities|Time|SetTimerbyEvent (delegate Custom|HitstunTimer) 0.5)))

(event Custom|WanderUntilTarget
  ;[1 0.8198 0.8198 1 32] Wait Outside of Player's Range
  ;;[1 1 1] Wander Until Target is Found
  (Variables|Default|SetisWandering true)
  (Variables|Targetting|SetHeroTarget 0)
  (CallFunction|FaceMovement)
  (bind _randomlocation (Class|NavigationSystemV1|GetRandomLocationinNavigableRadius (Transformation|GetActorLocation) (Variables|Default|GetwanderRadius) (Variables|Default|GetNavData) "/Game/Enemies/_Core/NavFilter_NoJumping.NavFilter_NoJumping_C"))
  (AI|AIMoveTo self _randomlocation 0 5.0 false
    (:then
      (bind _returnvalue (Utilities|Time|SetTimerbyEvent (delegate Custom|CheckRadiusWhileWandering) 0.3 true)))
    (:OnSuccess
      (if (Variables|Default|GetisWandering) :!label _label
        (Utilities|FlowControl|Delay 2.0)
        (Utilities|IsValid (Variables|Targetting|GetHeroTarget)
          (:Is%20Not%20Valid
            (CallFunction|WanderUntilTarget)))))
    (:OnFail
      (goto _label))))

(event Custom|InWaitRange
  ;[1 0.8198 0.8198 1 32] Wait Outside of Player's Range
  (CallFunction|OnlyFaceTarget)
  (bind _returnvalue (Utilities|Time|SetTimerbyEvent (delegate Custom|InWaitRangePositioning) 0.05 true))
  (Variables|Targetting|SetwaitingInRange true)
  (CallFunction|RequestAggroTimer)
  (bind _returnvalue_2 (Utilities|Time|SetTimerbyEvent (delegate Custom|RequestAggroTimer) 2.0 true)))

(event Custom|InWaitRangePositioning
  (bind _returnvalue (Transformation|GetActorLocation))
  (bind _herotarget (Variables|Targetting|GetHeroTarget))
  (bind _returnvalue_2 (Transformation|GetActorLocation _herotarget))
  (bind _returnvalue_3 (Math|Vector|Distance(Vector) _returnvalue_2 _returnvalue))
  ;[1 0.8198 0.8198 1 32] Wait Outside of Player's Range
  ;;[1 1 1] In Wait Range Positioning Movement
  (Utilities|IsValid (Variables|Targetting|GetHeroTarget)
    (:Is%20Valid
      (if (not (Variables|Default|GetinHitstun))
        (if (< _returnvalue_3 (Variables|Targetting|GetwaitRangeRadius)) ; If player is approaching
          ;;;[1 1 1] Back Away
          (|BackAwayGraph)
          (else
            ;;;[1 1 1] Move closer
            (if (> _returnvalue_3 (Variables|Targetting|GetwaitRangeRadius)) ; If player is fleeing
              (Utilities|Time|ClearandInvalidateTimerbyHandle (stale Custom|InWaitRange _returnvalue))
              (Variables|Targetting|SetwaitingInRange false)
              (CallFunction|WalktoWaitRange))))))))

(event Custom|StopAggro
  ;[1 1 1 1 32] Aggro State
  ;;[1 0.7115 0.7115] Leave Aggro State
  (Variables|Default|SetisAggro false)
  (Utilities|Time|ClearandInvalidateTimerbyHandle (stale Custom|AggroApproach _returnvalue))
  (Utilities|IsValid (Variables|Targetting|GetHeroTarget)
    (:Is%20Valid
      (Class|BIArrayEditEnemyWaiting|ArrayEditEnemyArray(Message) (Variables|Targetting|GetHeroTarget) true self true)
      (CallFunction|ApproachTarget))))

(event Custom|ApproachTarget
  ;[1 1 1] Activation
  (switch Utilities|FlowControl|Switch|SwitchonE_EnemyTypes (Variables|Default|GetenemyType)
    (:NewEnumerator0
      _)
    (:NewEnumerator1
      _))
  (CallFunction|WalktoWaitRange))

(event Custom|StopInWaitTimer
  ;[1 0.8198 0.8198 1 32] Wait Outside of Player's Range
  ;;[1 1 1] Stop Wait Timers
  (Utilities|Time|ClearandInvalidateTimerbyHandle (stale Custom|InWaitRange _returnvalue))
  (Utilities|Time|ClearandInvalidateTimerbyHandle (stale Custom|InWaitRange _returnvalue_2))
  (Variables|Targetting|SetwaitingInRange false))

(event Custom|ChooseAttack
  ;[1 1 1 1 32] Aggro State
  ;;[1 1 1] Attack State
  (switch int (Math|Random|RandomIntegerinRange 0 2)
    (:Default
      (Variables|Default|SetenemyState "NewEnumerator3" :!label _label)
      (CallFunction|AttackPunch))
    (:0
      (Variables|Default|SetenemyState "NewEnumerator2")
      (CallFunction|AttackHook))
    (:1
      (goto _label))
    (:2
      (Variables|Default|SetenemyState "NewEnumerator4")
      (CallFunction|AttackHeadbutt))))

(event Custom|AttackHook
  ;[1 1 1] Hook
  (if (Utilities|Enum|Equal(Enum) (Variables|Hitbox|GetattackState) "NewEnumerator0") ; If player is not attacking.
    (Variables|Hitbox|SetattackState "NewEnumerator1") ; set state to attacking
    ;;[1 1 1] Hitbox
    (CallFunction|SpawnHitbox (Math|Transform|MakeTransform "50.000000,0.000000,0.000000" "0, 0, 0" "3.000000,1.500000,3.000000") (Variables|Attack1|GethitboxLife_A1) (Variables|Attack1|Getdamage_A1) 0.5)
    (Development|PrintString "Hook attack!" false true "(R=0.000000,G=0.660000,B=1.000000,A=1.000000)" 5.0)
    (Utilities|Time|SetTimerbyEvent (delegate Custom|ResetAttackState) (Variables|Attack1|GetafterAttackCooldown_A1)) ; Set to idle after attack and cooldown are done.
  ))

(event Custom|AttackPunch
  ;[1 1 1] Punch
  (if (Utilities|Enum|Equal(Enum) (Variables|Hitbox|GetattackState) "NewEnumerator0") ; If player is not attacking.
    (Variables|Hitbox|SetattackState "NewEnumerator1") ; set state to attacking
    ;;[1 1 1] Hitbox
    (CallFunction|SpawnHitbox (Math|Transform|MakeTransform "50.000000,0.000000,0.000000" "0, 0, 0" "3.000000,1.500000,3.000000") (Variables|Attack2|GethitboxLife_A2) (Variables|Attack2|Getdamage_A2) 0.7)
    (Development|PrintString "Punch attack!" false true "(R=0.000000,G=0.660000,B=1.000000,A=1.000000)" 5.0)
    (Utilities|Time|SetTimerbyEvent (delegate Custom|ResetAttackState) (Variables|Attack2|GetafterAttackCooldown_A2)) ; Set to idle after attack and cooldown are done.
  ))

(event Custom|AttackHeadbutt
  ;[1 1 1] Headbutt
  (if (Utilities|Enum|Equal(Enum) (Variables|Hitbox|GetattackState) "NewEnumerator0") ; If player is not attacking.
    (Variables|Hitbox|SetattackState "NewEnumerator1") ; set state to attacking
    ;;[1 1 1] Hitbox
    (CallFunction|SpawnHitbox (Math|Transform|MakeTransform "50.000000,0.000000,0.000000" "0, 0, 0" "3.000000,1.500000,3.000000") (Variables|Attack3|GethitboxLife_A3) (Variables|Attack3|Getdamage_A3) 0.4)
    (Development|PrintString "Headbutt attack!" false true "(R=0.000000,G=0.660000,B=1.000000,A=1.000000)" 5.0)
    (Utilities|Time|SetTimerbyEvent (delegate Custom|ResetAttackState) (Variables|Attack3|GetafterAttackCooldown_A3)) ; Set to idle after attack and cooldown are done.
  ))

(event Custom|SpawnHitbox
  (params (RelativeTransform :type Transform) (Hitbox%20Lifetime :type Float%20%28double-precision%29) (Hitbox%20Damage :type Float%20%28double-precision%29) (InitialHitboxDelay :type Float%20%28double-precision%29))
  ;[1 1 1 1 32] Spawn Hitbox
  (Utilities|FlowControl|Delay InitialHitboxDelay)
  (if (Variables|Default|GetinHitstun)
    (Variables|Hitbox|SetattackState "NewEnumerator1")
    (Variables|Default|SetenemyState "NewEnumerator0")
    (else
      (bind _returnvalue (Game|AddComponentbyClass "/Script/Engine.BoxComponent" false RelativeTransform))
      (Variables|Hitbox|SetcurrentHitboxDamage Hitbox%20Damage)
      (Variables|/Script/Engine.ActorComponent|SetComponentTags _returnvalue (Variables|Hitbox|GetHitboxTags))
      (Transformation|AddRelativeLocation _returnvalue (.Location (Math|Transform|BreakTransform RelativeTransform)) false false)
      (Collision|SetCollisionResponsetoAllChannels _returnvalue "ECR_Overlap")
      (Utilities|FlowControl|Delay Hitbox%20Lifetime)
      (Utilities|IsValid _returnvalue
        (:Is%20Valid
          (Components|DestroyComponent _returnvalue))))))

(event Custom|CheckAttackState
  (bind _returnvalue (Transformation|GetActorLocation))
  (bind _herotarget (Variables|Targetting|GetHeroTarget))
  (bind _attackrange (Variables|Default|GetattackRange))
  (bind _returnvalue_2 (Transformation|GetActorLocation _herotarget))
  (bind _returnvalue_3 (Math|Vector|Distance2D(Vector) _returnvalue_2 _returnvalue))
  ;[1 1 1 1 32] Aggro State
  ;;[1 1 1] Check Aggro State
  (if (Variables|Default|GetinHitstun)
    (Utilities|Time|SetTimerbyEvent (delegate Custom|CheckAttackState) 0.5) ; Checks aggro state after hitstun done.
    (else
      (Utilities|IsValid (Variables|Targetting|GetHeroTarget)
        (:Is%20Valid
          (if (<= _returnvalue_3 (+ _attackrange (* _attackrange 0.3))) ; If still within attack range.
            (if (Utilities|Enum|Equal(Enum) (Variables|Hitbox|GetattackState) "NewEnumerator1")
              (Variables|Hitbox|SetattackState "NewEnumerator0")
              (CallFunction|ChooseAttack)
              (else
                (Development|PrintString "Oni Stuck #2")))
            (elif (<= _returnvalue_3 5e+02) ; IF still within aggro range
              (if (Utilities|Enum|Equal(Enum) (Variables|Hitbox|GetattackState) "NewEnumerator1")
                (Variables|Hitbox|SetattackState "NewEnumerator0")
                (CallFunction|AggroApproach)
                (else
                  (Development|PrintString "Oni stuck #1")))
              (else
                (Variables|Default|SetisAggro false)
                (if (Utilities|Enum|NotEqual(Enum) (Variables|Hitbox|GetattackState) "NewEnumerator1")
                  _
                  (else
                    (Variables|Hitbox|SetattackState "NewEnumerator0")))
                (CallFunction|StopAggro)
                (CallFunction|ChooseClosestTarget false (Variables|Targetting|GetHeroTarget))
                (CallFunction|ApproachTarget)))))))))

(event Custom|CheckRadiusWhileWandering
  (bind _charactermovement (Variables|Character|GetCharacterMovement))
  ;[1 0.8198 0.8198 1 32] Wait Outside of Player's Range
  ;;[1 1 1] Wander Until Target is Found
  (if (Variables|Default|GetisWandering)
    (for _array_element (Variables|Default|GetHeroes)
      (Utilities|IsValid _array_element
        (:Is%20Valid
          (if (<= (Math|Vector|VectorLengthXY (- (Transformation|GetActorLocation _array_element) (Transformation|GetActorLocation))) 1.8e+03)
            (Utilities|Time|ClearandInvalidateTimerbyHandle (stale Custom|WanderUntilTarget _returnvalue))
            (Variables|Default|SetisWandering false)
            (Components|Movement|StopMovementImmediately _charactermovement)
            (Variables|/Script/Engine.MovementComponent|SetVelocity _charactermovement (Pawn|Components|CharacterMovement|GetLastUpdateVelocity _charactermovement))
            (CallFunction|ChooseClosestTarget false)
            (CallFunction|WalktoWaitRange)))))
    (else
      (Utilities|Time|ClearandInvalidateTimerbyHandle (stale Custom|WanderUntilTarget _returnvalue)))))

(event Custom|HitstunTimer
  ;[1 1 1] Hitstun
  (Variables|Default|SetinHitstun false)
  (Variables|Hitbox|SetattackState "NewEnumerator1"))

(event Custom|RequestAggroTimer
  ;[1 0.8198 0.8198 1 32] Wait Outside of Player's Range
  (Utilities|IsValid (Variables|Targetting|GetHeroTarget)
    (:Is%20Valid
      (Class|BIRequestAggro|RequestAggro(Message) (Variables|Targetting|GetHeroTarget) self))))

(event Custom|WalkToWaitRange
  ;[1 0.8198 0.8198 1 32] Wait Outside of Player's Range
  (CallFunction|FaceMovement)
  (|WalkTowardsWaitRangeGraph))

(event Custom|Attack_PunchingBag)

(event Custom|Attack_Sneak)

(event Custom|AggroApproach
  ;[1 1 1 1 32] Aggro State
  ;;[1 1 1] Aggro Approach
  (CallFunction|OnlyFaceTarget)
  (bind _returnvalue (Utilities|Time|SetTimerbyEvent (delegate Custom|CheckAttackState) 0.5 true)) ; Checks aggro state when chasing
  (if (not (Variables|Default|GetinHitstun))
    (AI|AIMoveTo self "0, 0, 0" (Variables|Targetting|GetHeroTarget) (Variables|Default|GetattackRange) false
      (:OnSuccess
        (CallFunction|ChooseAttack)
        (Utilities|Time|ClearandInvalidateTimerbyHandle _returnvalue))
      (:OnFail
        (CallFunction|ChooseClosestTarget false (Variables|Targetting|GetHeroTarget))
        (CallFunction|StopAggro)))))

(event Custom|Activate
  ;[1 1 1] Activation
  (CallFunction|ChooseClosestTarget false)
  (switch Utilities|FlowControl|Switch|SwitchonE_EnemyTypes (Variables|Default|GetenemyType)
    (:NewEnumerator0
      _)
    (:NewEnumerator1
      _))
  (CallFunction|WanderUntilTarget))

(event EventGetHitboxDamage
  (params (ActorToDamage :type Actor%20Object%20Reference))
  ;[1 1 1 1 32] Take Damage
  (Class|BISendHitboxDamage|SendHitboxDamage(Message) ActorToDamage (Variables|Hitbox|GetcurrentHitboxDamage)))

(event EventSendHitboxDamage
  (params (HitboxDamage :type Float%20%28double-precision%29))
  (bind _satoshigrappleactor (Variables|Default|GetsatoshiGrappleActor))
  ;[1 1 1 1 32] Take Damage
  (Variables|CharacterSettings|Sethealth (- (Variables|CharacterSettings|Gethealth) HitboxDamage))
  (Rendering|Components|TextRender|SetText (Variables|Default|GetHealthDebug) (Utilities|Text|ToText(Float) (Variables|CharacterSettings|Gethealth) "HalfToEven"))
  ;[1 1 1] Death
  (if (or (<= (Variables|CharacterSettings|Gethealth) 0.0) (Math|Float|NearlyEqual(Float) (Variables|CharacterSettings|Gethealth) 0.0 0.001)) ; If enemy has died.
    (Utilities|IsValid (Variables|Targetting|GetHeroTarget)
      (:Is%20Valid
        (Class|BIArrayEditEnemyWaiting|ArrayEditEnemyArray(Message) (Variables|Targetting|GetHeroTarget) true self false)
        (Class|BIArrayEditEnemyWaiting|ArrayEditEnemyArray(Message) (Variables|Targetting|GetHeroTarget) true self true))
      (:Is%20Not%20Valid
        _))
    (Variables|Default|SetenemyState "NewEnumerator5")
    (Variables|/Script/Engine.CharacterMovementComponent|SetMaxWalkSpeed (Variables|Character|GetCharacterMovement) 0.0)
    (Variables|Targetting|SetfaceTarget false)
    (Collision|SetCollisionResponsetoChannel (Variables|Default|GetHurtBox) "ECC_WorldDynamic" "ECR_Ignore")
    (Utilities|IsValid _satoshigrappleactor
      (:Is%20Valid
        (Default|GrappleDisable _satoshigrappleactor))
      (:Is%20Not%20Valid
        _))
    (Utilities|FlowControl|Delay 2.0)
    (Actor|DestroyActor)
    (else
      ;[1 1 1] Hitstun
      (if (!= (Variables|Default|GetlastOffendingActor) "/Game/Characters/Satoshi/BP_PlayerSatoshi.BP_PlayerSatoshi")
        (CallFunction|ApplyHitstun)
        (Components|Movement|StopMovementImmediately (Variables|Character|GetCharacterMovement))))))

(event EventBeginPlay
  ;[1 1 1] Begin Play
  (bind _outactors (Actor|GetAllActorswithTag "Hero"))
  (Variables|Default|SetHeroes _outactors)
  (bind _outactors_2 (Actor|GetAllActorsOfClass "/Script/NavigationSystem.RecastNavMesh"))
  (Variables|Default|SetNavData (Utilities|Array|Get(acopy) _outactors_2))
  (Variables|Default|SetwanderCenter (Transformation|GetActorLocation))
  (CallFunction|Activate)
  (Rendering|Components|TextRender|SetText (Variables|Default|GetHealthDebug) (Utilities|Text|ToText(Float) (Variables|CharacterSettings|Gethealth) "HalfToEven"))
  (bind _returnvalue (Actor|GetActorOfClass "/Game/Camera/BP_Camera.BP_Camera_C"))
  (Variables|Default|SetCam (Variables|/Game/Camera/BP_Camera.BP_Camera_C|GetCamera _returnvalue)))

(event EventUpdatePlayer
  (params (NewPlayerPawn :type Pawn%20Object%20Reference))
  (if (!= (Variables|Targetting|GetHeroTarget) 0)
    (Variables|Targetting|SetHeroTarget NewPlayerPawn)
    (bind _outactors (Actor|GetAllActorswithTag "Hero"))
    (Variables|Default|SetHeroes _outactors)))

(event EventSatoshiGrapple
  (params (GrappleActor :type BP%20Satoshi%20Grapple%20Object%20Reference) (SatoshiGrappleActor :type BP%20Player%20Satoshi%20Object%20Reference))
  (Class|BPIRecieveGrappleLocation|RecieveGrappleMesh(Message) GrappleActor (Variables|Character|GetMesh))
  (Variables|Default|SetsatoshiGrappleActor SatoshiGrappleActor)
  (CallFunction|FaceMovement)
  (CallFunction|ChooseRandomTarget))

(event EventTick
  (params (DeltaSeconds :type Float%20%28single-precision%29))
  ;[1 1 1] Event Tick
  (if (Variables|Targetting|GetfaceTarget)
    (Utilities|IsValid (Variables|Targetting|GetHeroTarget)
      (:Is%20Valid
        (Transformation|SetActorRotation (Math|Rotator|MakeRotator 0.0 0.0 (.yaw (Math|Rotator|FindLookatRotation (Transformation|GetActorLocation) (Transformation|GetActorLocation (Variables|Targetting|GetHeroTarget)))))))
      (:Is%20Not%20Valid
        _)))
  ;[1 1 1] Idle Anim State
  (if (Utilities|Enum|NotEqual(Enum) (Variables|Hitbox|GetattackState) "NewEnumerator0")
    _
    (elif (>= (Math|Vector|VectorLengthXY (Variables|/Script/Engine.MovementComponent|GetVelocity (Variables|Character|GetCharacterMovement))) 2e+01)
      (Variables|Default|SetenemyState "NewEnumerator1")
      (else
        (Variables|Default|SetenemyState "NewEnumerator0"))))
  (Development|PrintString (Utilities|String|EnumtoString (Variables|Hitbox|GetattackState)) false true "(R=1.000000,G=0.240935,B=0.272776,A=1.000000)" 2.0 "stun")
  (Transformation|SetWorldRotation (Variables|Default|GetHealthDebug) (Math|Rotator|FindLookatRotation (Transformation|GetActorLocation) (Transformation|GetWorldLocation (Variables|Default|GetCam))) false false))

(event EventPermitAggro
  ;[1 1 1 1 32] Aggro State
  ;;[1 1 1] Aggro Permitted
  (CallFunction|StopinWaitTimer)
  (Development|PrintString (Utilities|String|Append (Utilities|GetDisplayName self) " is turning aggro!") false)
  (Variables|Default|SetisAggro true)
  (CallFunction|AggroApproach))

(event EventCheckDeath
  (params (callingActor :type Actor%20Object%20Reference))
  (bind _health (Variables|CharacterSettings|Gethealth))
  ;[1 1 1] Death
  (Class|BPIReturnDeath|ReturnDeath(Message) callingActor self (or (<= _health 0.0) (Math|Float|NearlyEqual(Float) _health 0.0 0.001))))

(fn ConstructionScript
  (Variables|/Script/Engine.CharacterMovementComponent|SetMaxWalkSpeed (Variables|Character|GetCharacterMovement) (Variables|CharacterSettings|GetwalkSpeed)))

(fn OnlyFaceTarget
  (Variables|Targetting|SetfaceTarget true)
  (Variables|/Script/Engine.CharacterMovementComponent|SetbOrientRotationToMovement (Variables|Character|GetCharacterMovement) false)
  (Variables|/Script/Engine.CharacterMovementComponent|SetbUseControllerDesiredRotation (Variables|Character|GetCharacterMovement) false))

(fn FaceMovement
  (Variables|Targetting|SetfaceTarget false)
  (Variables|/Script/Engine.CharacterMovementComponent|SetbOrientRotationToMovement (Variables|Character|GetCharacterMovement) true)
  (Variables|/Script/Engine.CharacterMovementComponent|SetbUseControllerDesiredRotation (Variables|Character|GetCharacterMovement) true))

(fn IsNotGrappleSatoshi
  (params (FoundActor :type Actor%20Object%20Reference))
  (Utilities|IsValid FoundActor
    (:Is%20Valid
      (if (Actor|ActorHasTag FoundActor "Satoshi")
        (bind _asbp_player_satoshi (Utilities|Casting|CastToBP_PlayerSatoshi FoundActor)
          (:then
            (if (Variables|/Game/Characters/Satoshi/BP_PlayerSatoshi.BP_PlayerSatoshi_C|GetinGrapple _asbp_player_satoshi)
              (return true)
              (else
                _)))
          (:CastFailed
            _))))
    (:Is%20Not%20Valid
      _))
  (return false))

(event OnSeePawn(PawnSensing)
  (params (Pawn :type Pawn%20Object%20Reference))
  (bind _charactermovement (Variables|Character|GetCharacterMovement))
  ;[1 0.549 0.5765 1 32] Choose Target
  ;;[1 0.4745 0.4745] Retarget on Sight
  (if (not (Variables|Targetting|GetonSeePawnCooldownFlag)) ; If retarget cooldown has ended.
    (if (Actor|ActorHasTag Pawn "Hero") ; If is a hero
      (if (!= Pawn (Variables|Targetting|GetHeroTarget)) ; Is not their current target
        (if (not (CallFunction|IsNotGrappleSatoshi Pawn))
          (Utilities|IsValid (Variables|Targetting|GetHeroTarget)
            (:Is%20Valid
              (if (> (Math|Vector|Distance(Vector) (Transformation|GetActorLocation Pawn) (Transformation|GetActorLocation (Variables|Targetting|GetHeroTarget))) 2e+02) ; Is far enough away from current target
                (CallFunction|ChangeHeroTarget Pawn :!label _label)
                (Variables|Targetting|SetwaitingInRange false)
                (Variables|Default|SetisWandering false)
                (CallFunction|StopinWaitTimer) ; Here more as a precaution
                (if (Math|Float|NearlyEqual(Float) (.z (Variables|/Script/Engine.MovementComponent|GetVelocity (Variables|Character|GetCharacterMovement))) 0.0 1e-05)
                  (Components|Movement|StopMovementImmediately _charactermovement)
                  (Variables|/Script/Engine.MovementComponent|SetVelocity _charactermovement (Pawn|Components|CharacterMovement|GetLastUpdateVelocity _charactermovement)))
                (CallFunction|ApproachTarget)
                (Variables|Targetting|SetonSeePawnCooldownFlag true)
                (Utilities|Time|SetTimerbyEvent (delegate Custom|RetargetCooldown) 5.0)))
            (:Is%20Not%20Valid
              (goto _label))))))))

(event Custom|ChangeHeroTarget
  (params (NewHeroTarget :type Actor%20Object%20Reference))
  ;[1 0.549 0.5765 1 32] Change Hero Target
  (Utilities|IsValid (Variables|Targetting|GetHeroTarget)
    (:Is%20Valid
      (Class|BIArrayEditEnemyWaiting|ArrayEditEnemyArray(Message) (Variables|Targetting|GetHeroTarget) true self false)
      (Class|BIArrayEditEnemyWaiting|ArrayEditEnemyArray(Message) (Variables|Targetting|GetHeroTarget) true self true)
      (Utilities|IsValid NewHeroTarget
        (:Is%20Valid
          (Class|BIArrayEditEnemyWaiting|ArrayEditEnemyArray(Message) NewHeroTarget false self false :!label _label))
        (:Is%20Not%20Valid
          _)))
    (:Is%20Not%20Valid
      (goto _label)))
  (Variables|Targetting|SetHeroTarget NewHeroTarget))

(event Custom|RetargetCooldown
  ;[1 0.549 0.5765 1 32] Choose Target
  ;;[1 0.4745 0.4745] Retarget on Sight
  (Variables|Targetting|SetonSeePawnCooldownFlag false))

(event Custom|ChooseClosestTarget
  (params (ExcludePreviousTarget :type Boolean) (PreviousTarget :type Actor%20Object%20Reference))
  ;[1 0.549 0.5765 1 32] Choose Target
  ;;[1 0.4745 0.4745] Choose Closest Target
  (Variables|Targetting|SetchooseHeroDistanceCheck 1e+08)
  (for _array_element (Variables|Default|GetHeroes)
    (Utilities|IsValid _array_element
      (:Is%20Valid
        (if (< (Math|Vector|Distance(Vector) (Transformation|GetActorLocation _array_element) (Transformation|GetActorLocation)) (Variables|Targetting|GetchooseHeroDistanceCheck))
          (if (.ReturnValue (AI|Navigation|ProjectPointtoNavigation (Transformation|GetActorLocation _array_element) (Variables|Default|GetNavData) 0 "0.000000,0.000000,300.000000")) ; If hero is reachable
            (if ExcludePreviousTarget
              (if (!= PreviousTarget _array_element)
                (Variables|Targetting|SetchooseHeroDistanceCheck (Math|Vector|Distance(Vector) (Transformation|GetActorLocation _array_element) (Transformation|GetActorLocation)) :!label _label)
                (CallFunction|ChangeHeroTarget _array_element))
              (else
                (goto _label))))))))
  ;;[1 0.4745 0.4745] Wander if no target is found
  (Utilities|IsValid (Variables|Targetting|GetHeroTarget)
    (:Is%20Valid
      (if (not (.ReturnValue (AI|Navigation|ProjectPointtoNavigation (Transformation|GetActorLocation (Variables|Targetting|GetHeroTarget)) (Variables|Default|GetNavData) 0 "0.000000,0.000000,300.000000")))
        (Variables|Default|SetwanderCenter (Transformation|GetActorLocation) :!label _label_2)
        (CallFunction|WanderUntilTarget)))
    (:Is%20Not%20Valid
      (goto _label_2))))

(event Custom|ChooseRandomTarget
  (bind _heroes (Variables|Default|GetHeroes))
  (bind _outitem (Utilities|Array|Random _heroes))
  ;[1 0.549 0.5765 1 32] Choose Target
  ;;[1 0.4745 0.4745] Choose Random Target
  (if (CallFunction|IsNotGrappleSatoshi _outitem)
    (Utilities|FlowControl|Delay 0.05)
    (CallFunction|ChooseRandomTarget)
    (else
      (CallFunction|ChangeHeroTarget _outitem)
      ;;[1 0.4745 0.4745] Wander if no target is found
      (Utilities|IsValid (Variables|Targetting|GetHeroTarget)
        (:Is%20Valid
          (if (not (.ReturnValue (AI|Navigation|ProjectPointtoNavigation (Transformation|GetActorLocation (Variables|Targetting|GetHeroTarget)) (Variables|Default|GetNavData) 0 "0.000000,0.000000,300.000000")))
            (Variables|Default|SetwanderCenter (Transformation|GetActorLocation) :!label _label)
            (CallFunction|WanderUntilTarget)))
        (:Is%20Not%20Valid
          (goto _label))))))