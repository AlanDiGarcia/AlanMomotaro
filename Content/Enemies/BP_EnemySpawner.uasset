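; Enemy spawner that, once when a Hero-tagged actor overlaps its box, spawns a set number of enemies with default AI controllers.
; SpawnType selects either listed locations projected onto the navmesh, reusing random entries beyond the list's length, or random reachable points around the spawner.
; Radius mode retries next tick until a point clears the inner threshold, but spawns at a freshly rolled point, so that minimum distance is not guaranteed.
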(event OnComponentBeginOverlap(Box)
  (params (OverlappedComponent :type Primitive%20Component%20Object%20Reference) (OtherActor :type Actor%20Object%20Reference) (OtherComp :type Primitive%20Component%20Object%20Reference) (OtherBodyIndex :type Integer) (bFromSweep :type Boolean) (SweepResult :type Hit%20Result%20Structure%20%28by%20ref%29))
  (if (Actor|ActorHasTag OtherActor "Hero")
    (Utilities|FlowControl|DoOnce false
      (:Completed
        (CallFunction|SpawnEnemy)))))

(event Custom|SpawnEnemy
  (bind _returnvalue (Transformation|GetActorTransform))
  (bind _spawnlocations (Variables|SpawnAtLocation|GetspawnLocations))
  (switch Utilities|FlowControl|Switch|SwitchonE_SpawnType (Variables|Default|GetspawnType)
    (:NewEnumerator0
      ;[1 1 1] Spawn at Location
      (bind _returnvalue_2 (Actor|GetActorOfClass "/Script/NavigationSystem.RecastNavMesh"))
      (for _index (range 0 (- (Variables|Default|GetspawnAmount) 1))
        (if (> _index (- (Utilities|Array|Length _spawnlocations) 1)) ; If index is greater than amount in array.
          (bind _returnvalue_3 (AI|SpawnAIFromClass (Variables|Default|GetenemyToSpawn) 0 (.ProjectedLocation (AI|Navigation|ProjectPointtoNavigation (.OutItem (Utilities|Array|Random _spawnlocations)) 0 0 "0.000000,0.000000,500.000000")) "0, 0, 0" false 0))
          (Pawn|SpawnDefaultController _returnvalue_3)
          (else
            (bind _returnvalue_4 (AI|SpawnAIFromClass (Variables|Default|GetenemyToSpawn) 0 (.ProjectedLocation (AI|Navigation|ProjectPointtoNavigation (Utilities|Array|Get(acopy) _spawnlocations _index) _returnvalue_2 0 "0.000000,0.000000,500.000000")) "0, 0, 0" false 0))
            (Pawn|SpawnDefaultController _returnvalue_4)))))
    (:NewEnumerator1
      ;[1 1 1] Spawn in Radius
      (Variables|SpawnInRadius|SetspawnRadiusIndex 0)
      (bind _returnvalue_5 (Actor|GetActorOfClass "/Script/NavigationSystem.RecastNavMesh"))
      (if (< (Variables|SpawnInRadius|GetspawnRadiusIndex) (Variables|Default|GetspawnAmount)) :!label _label
        (if (>= (Math|Vector|Distance2D(Vector) (.RandomLocation (AI|Navigation|GetRandomReachablePointinRadius (.location _returnvalue) (Variables|SpawnInRadius|GetspawnRadius_OuterThreshold) _returnvalue_5 0)) (Transformation|GetActorLocation)) (Variables|SpawnInRadius|GetspawnRadius_InnerThreshold)) :!label _label_2
          (Math|Integer|IncrementInt (Variables|SpawnInRadius|GetspawnRadiusIndex)
            (:%20%20
              (bind _returnvalue_6 (AI|SpawnAIFromClass (Variables|Default|GetenemyToSpawn) 0 (.RandomLocation (AI|Navigation|GetRandomReachablePointinRadius (.location _returnvalue) (Variables|SpawnInRadius|GetspawnRadius_OuterThreshold) _returnvalue_5 0)) (.rotation _returnvalue) false 0))
              (Pawn|SpawnDefaultController _returnvalue_6)
              (goto _label)))
          (else
            (Utilities|FlowControl|DelayUntilNextTick)
            (goto _label_2)))))))

(fn ConstructionScript)