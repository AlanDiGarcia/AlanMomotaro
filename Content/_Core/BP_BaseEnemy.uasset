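; Base enemy character that trades hitbox damage with players and applies its walk speed at construction.
; HurtBox overlaps with hero-tagged components request damage through interface messages, which reduce Health and update a debug text.
; SpawnHitbox creates temporary tagged box components and stores their damage for the attacker to send on request.
; Two three-hit combo chains with timer resets exist but are disconnected, leaving Attack1 and Attack2 empty.
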(event OnComponentBeginOverlap(HurtBox)
  (params (OverlappedComponent :type Primitive%20Component%20Object%20Reference) (OtherActor :type Actor%20Object%20Reference) (OtherComp :type Primitive%20Component%20Object%20Reference) (OtherBodyIndex :type Integer) (bFromSweep :type Boolean) (SweepResult :type Hit%20Result%20Structure%20%28by%20ref%29))
  ;[1 1 1 1 32] Take Damage
  (if (Components|ComponentHasTag OtherComp (Variables|Default|GetHeroHitboxTagName)) ; If hurtbox was overlapped by hostile hitbox.
    (Class|BIGetHitboxDamage|GetHitboxDamage(Message) OtherActor self)))

(event Custom|ResetAttackState
  ;[1 1 1] Reset to Idle After Attack
  (Variables|Default|SetattackState "NewEnumerator0")
  (if (>= (Variables|Attack1|GetattackComboCounter_A1) 3)
    (Variables|Attack1|SetattackComboCounter_A1 0))
  (if (>= (Variables|Attack2|GetattackComboCounter_A2) 3)
    (Variables|Attack2|SetattackComboCounter_A2 0)))

(event Custom|Attack2CombCheck
  ;[1 1 1] Attack 2
  ;;[1 1 1] Attack 2 Combo Check
  (if (not (Utilities|Enum|Equal(Enum) (Variables|Default|GetattackState) "NewEnumerator2"))
    (Variables|Attack2|SetattackComboCounter_A2 0)))

(event Custom|SpawnHitbox
  (params (RelativeTransform :type Transform) (Hitbox%20Lifetime :type Float%20%28double-precision%29) (Hitbox%20Damage :type Float%20%28double-precision%29))
  ;[1 1 1 1 32] Spawn Hitbox
  (bind _returnvalue (Game|AddComponentbyClass "/Script/Engine.BoxComponent" false RelativeTransform))
  (Variables|Default|SetcurrentHitboxDamage Hitbox%20Damage)
  (Variables|/Script/Engine.ActorComponent|SetComponentTags _returnvalue (Variables|Default|GetHitboxTags))
  (Transformation|AddRelativeLocation _returnvalue (.Location (Math|Transform|BreakTransform RelativeTransform)) false false)
  (Collision|SetCollisionResponsetoAllChannels _returnvalue "ECR_Overlap")
  (Utilities|FlowControl|Delay Hitbox%20Lifetime)
  (Components|DestroyComponent _returnvalue))

(event Custom|Attack1ComboCheck
  ;[1 1 1] Attack 1
  ;;[1 1 1] Attack 1 Combo Check
  (if (not (Utilities|Enum|Equal(Enum) (Variables|Default|GetattackState) "NewEnumerator1"))
    (Variables|Attack1|SetattackComboCounter_A1 0)))

(event EventGetHitboxDamage
  (params (ActorToDamage :type Actor%20Object%20Reference))
  ;[1 1 1 1 32] Take Damage
  (Class|BISendHitboxDamage|SendHitboxDamage(Message) ActorToDamage (Variables|Default|GetcurrentHitboxDamage)))

(event EventSendHitboxDamage
  (params (HitboxDamage :type Float%20%28double-precision%29))
  ;[1 1 1 1 32] Take Damage
  (Variables|CharacterSettings|Sethealth (- (Variables|CharacterSettings|Gethealth) HitboxDamage))
  (Rendering|Components|TextRender|SetText (Variables|Default|GetHealthDebug) (Utilities|Text|ToText(Float) (* (Variables|CharacterSettings|Gethealth) 1e+02) "HalfToEven")))

(event EventAttack1
  ;[1 1 1] Attack 1
)

(event EventAttack2
  ;[1 1 1] Attack 2
)

(fn ConstructionScript
  (Variables|/Script/Engine.CharacterMovementComponent|SetMaxWalkSpeed (Variables|Character|GetCharacterMovement) (Variables|CharacterSettings|GetwalkSpeed)))