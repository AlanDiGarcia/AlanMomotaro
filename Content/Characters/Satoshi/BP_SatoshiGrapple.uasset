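; Short-lived grapple actor for Satoshi that detects an enemy and has the player move to it.
; On BeginPlay it finds BP_PlayerSatoshi via GetActorOfClass and starts a LifeTime timer to destroy itself.
; The first overlap with an "Enemy"-tagged actor plays a battle cry and sends that enemy SatoshiGrappleMessage with itself and the player.
; RecieveGrappleMesh takes an enemy mesh and forwards it to the player's MoveToGrapplePoint.
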(event OnComponentBeginOverlap(GrappleCollision)
  (params (OverlappedComponent :type Primitive%20Component%20Object%20Reference) (OtherActor :type Actor%20Object%20Reference) (OtherComp :type Primitive%20Component%20Object%20Reference) (OtherBodyIndex :type Integer) (bFromSweep :type Boolean) (SweepResult :type Hit%20Result%20Structure%20%28by%20ref%29))
  (if (Actor|ActorHasTag OtherActor "Enemy")
    (Utilities|FlowControl|DoOnce false
      (:Completed
        (Utilities|IsValid (Variables|Default|GetOwningActor)
          (:Is%20Valid
            (Audio|PlaySound2D "/Game/Sound/Voicelines/satoshivoice_battlecry.satoshivoice_battlecry" 1.0 1.0 0.0 0 0)
            (Class|BPISatoshiGrapple|SatoshiGrapple(Message) OtherActor self (Variables|Default|GetOwningActor)))
          (:Is%20Not%20Valid
            (Development|PrintString "Satoshi Grapple - Owning actor is not valid")))))))

(event Custom|Destroy
  (Actor|DestroyActor))

(event EventBeginPlay
  (bind _returnvalue (Actor|GetActorOfClass "/Game/Characters/Satoshi/BP_PlayerSatoshi.BP_PlayerSatoshi_C"))
  (Variables|Default|SetOwningActor _returnvalue)
  (Utilities|Time|SetTimerbyEvent (delegate Custom|Destroy) (Variables|Default|GetlifeTime)))

(event EventRecieveGrappleMesh
  (params (EnemyMesh :type Skeletal%20Mesh%20Component%20Object%20Reference))
  (Default|MovetoGrapplePoint (Variables|Default|GetOwningActor) EnemyMesh))

(fn ConstructionScript)