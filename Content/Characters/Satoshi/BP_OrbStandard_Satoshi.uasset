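; BP_OrbStandard_Satoshi is Satoshi's standard orb projectile, which self-destructs after a set lifetime and reports its damage through a hitbox message.
; Tick pushes the physics mesh along its launch direction, under a horizontal speed cap, while it has no target.
; AI Perception locks onto the first Enemy-tagged actor once, starting a looping timer that steers the orb with capped homing force.
; If that target becomes invalid, Tick thrust resumes along the last direction.
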(event OnTargetPerceptionUpdated(AIPerception)
  (params (Actor :type Actor%20Object%20Reference) (Stimulus :type AI%20Stimulus%20Structure))
  (if (Actor|ActorHasTag Actor "Enemy")
    (Utilities|FlowControl|DoOnce false
      (:Completed
        (Variables|Default|SettargetPawn Actor)
        (Utilities|Time|SetTimerbyEvent (delegate Custom|AimAssist) (Variables|Default|GetaimAssistCheck) true)))))

(event Custom|AimAssist
  (Utilities|IsValid (Variables|Default|GettargetPawn)
    (:Is%20Valid
      (bind _output_get (Variables|Default|SettargetDirection (Math|Rotator|GetRotationXVector (Math|Rotator|MakeRotator (.roll (Math|Rotator|FindLookatRotation (Transformation|GetActorLocation) (Transformation|GetActorLocation (Variables|Default|GettargetPawn)))) (.pitch (Math|Rotator|FindLookatRotation (Transformation|GetActorLocation) (Transformation|GetActorLocation (Variables|Default|GettargetPawn)))) (* (.yaw (Math|Rotator|FindLookatRotation (Transformation|GetActorLocation) (Transformation|GetActorLocation (Variables|Default|GettargetPawn)))) 1.0)))))
      (bind _returnvalue (Physics|GetPhysicsLinearVelocity (Variables|Default|GetMesh) "None"))
      (if (< (Math|Vector|VectorLengthXY _returnvalue) 3.5e+03)
        (Physics|AddForce (Variables|Default|GetMesh) (* _output_get (Variables|Default|GetaimAssistStrength)) "None" false)))
    (:Is%20Not%20Valid
      (Variables|Default|SettargetPawn 0))))

(event EventGetHitboxDamage
  (params (ActorToDamage :type Actor%20Object%20Reference))
  (Class|BISendHitboxDamage|SendHitboxDamage(Message) ActorToDamage (Variables|Default|GetorbDamage)))

(event EventTick
  (params (DeltaSeconds :type Float%20%28single-precision%29))
  (bind _returnvalue (Physics|GetPhysicsLinearVelocity (Variables|Default|GetMesh) "None"))
  (if (< (Math|Vector|VectorLengthXY _returnvalue) 3e+03)
    (Utilities|IsValid (Variables|Default|GettargetPawn)
      (:Is%20Not%20Valid
        (Physics|AddForce (Variables|Default|GetMesh) (* (Variables|Default|GettargetDirection) (Variables|Default|GetorbSpeed)) "None" false)))))

(event EventBeginPlay
  (Variables|Default|SettargetDirection (Transformation|GetActorForwardVector))
  (Utilities|FlowControl|Delay (Variables|Default|GetorbLifetime))
  (Actor|DestroyActor))

(fn ConstructionScript)