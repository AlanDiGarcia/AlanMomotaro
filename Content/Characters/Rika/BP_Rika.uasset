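; BP_Rika is the Rika character that the player can talk to.
; Overlapping its Box sets a "Press X to talk" text render and enables player input; no end-overlap handler reverses this.
; Pressing X plays Rika's welcome voice and shows a talk widget, then after a delay adds a Sleepytime widget with Momo's relief voice.
; The Inrange check is an empty branch, so it does not gate the interaction.
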(event OnComponentBeginOverlap(Box)
  (params (OverlappedComponent :type Primitive%20Component%20Object%20Reference) (OtherActor :type Actor%20Object%20Reference) (OtherComp :type Primitive%20Component%20Object%20Reference) (OtherBodyIndex :type Integer) (bFromSweep :type Boolean) (SweepResult :type Hit%20Result%20Structure%20%28by%20ref%29))
  (Rendering|Components|TextRender|SetText (Variables|Default|GetTextRender) (Utilities|Text|ToText(String) "Press X to talk"))
  (Input|EnableInput (Game|GetPlayerController 0))
  (if (Variables|Default|GetInrange)
    _))

(event EventBeginPlay)

(event EventTick
  (params (DeltaSeconds :type Float%20%28single-precision%29)))

(event Input|KeyboardEvents|X
  (params (Key :type Key%20Structure :default "None"))
  (:Pressed
    (Audio|PlaySound2D "/Game/Sound/Voicelines/rikavoice_welcome.rikavoice_welcome" 2.0 1.0 0.0 0 0)
    (bind _returnvalue (UserInterface|CreateWidget "/Game/_UI/TextBoxAssets/WB_TB_RikaTalk1.WB_TB_RikaTalk1_C"))
    (UserInterface|Viewport|AddtoViewport _returnvalue 0)
    (Utilities|FlowControl|Delay 2.0)
    (bind _returnvalue_2 (UserInterface|CreateWidget "/Game/_UI/WB_Sleepytime.WB_Sleepytime_C"))
    (UserInterface|Viewport|AddtoViewport _returnvalue_2 0)
    (Audio|PlaySound2D "/Game/Sound/Voicelines/momovoice_relief.momovoice_relief" 2.0 1.0 0.0 0 0)
    (Utilities|FlowControl|Delay 2.0)))

(fn ConstructionScript)