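; Camera target actor that smoothly follows the first player controller's controlled pawn.
; Shortly after BeginPlay, or whenever ChangeTarget is called, it caches that pawn as the follow target.
; Each Tick, while the target is valid, it interpolates its location toward the pawn with FInterpTo per axis, using separate speeds for horizontal and vertical movement.
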(event Custom|ChangeTarget
  (Variables|Default|SetPlayer (Pawn|GetControlledPawn (Game|GetPlayerController 0))))

(event EventBeginPlay
  (Utilities|FlowControl|Delay 0.3)
  (Variables|Default|SetPlayer (Pawn|GetControlledPawn (Game|GetPlayerController 0))))

(event EventTick
  (params (DeltaSeconds :type Float%20%28single-precision%29))
  (bind _returnvalue (Utilities|Time|GetWorldDeltaSeconds))
  (bind _returnvalue_2 (Transformation|GetActorLocation))
  (bind _player (Variables|Default|GetPlayer))
  (bind _interpspeedxy (Variables|Default|GetInterpSpeedXY))
  (bind _returnvalue_3 (Transformation|GetActorLocation _player))
  (Utilities|IsValid (Variables|Default|GetPlayer)
    (:Is%20Valid
      (Transformation|SetActorLocation (Math|Vector|MakeVector (Math|Interpolation|FInterpTo (.x _returnvalue_2) (.x _returnvalue_3) _returnvalue _interpspeedxy) (Math|Interpolation|FInterpTo (.y _returnvalue_2) (.y _returnvalue_3) _returnvalue _interpspeedxy) (Math|Interpolation|FInterpTo (.z _returnvalue_2) (.z _returnvalue_3) _returnvalue (Variables|Default|GetInterpSpeedZ))) false false))))

(fn ConstructionScript)