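; Player follow camera that places its SplineTarget component at the controlled pawn's location every tick, once a BP_CameraTarget is found.
; GetCameraRotation selects a fixed centered angle while the pawn moves, swinging it to either side when idle and facing along ±X.
; BeginPlay finds the BP_CameraTrack and computes a distance along its spline, but only abandoned, disconnected spline-steering experiments use that distance.
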(event EventBeginPlay
  ;[1 1 1] Safegaurd In Case Camera Track is not Set
  (Utilities|IsValid (Variables|Default|GetcameraTrack)
    (:Is%20Valid
      _)
    (:Is%20Not%20Valid
      (bind _returnvalue (Actor|GetActorOfClass "/Game/Camera/BP_CameraTrack.BP_CameraTrack_C"))
      (Variables|Default|SetcameraTrack _returnvalue)))
  (Utilities|FlowControl|Delay 0.2)
  ;[1 1 1] Cam Target
  (bind _returnvalue_2 (Actor|GetActorOfClass "/Game/Camera/BP_CameraTarget.BP_CameraTarget_C"))
  (Variables|Default|SetcamTarget _returnvalue_2)
  (Variables|Default|SetlastFrameAimVector (Math|Vector|GetForwardVector (Variables|Default|GetCamera)))
  (bind _distance (CallFunction|GetLocationsDistanceAlongSpline (Transformation|GetActorLocation (Variables|Default|GetcamTarget)) (Variables|/Game/Camera/BP_CameraTrack.BP_CameraTrack_C|GetSpline (Variables|Default|GetcameraTrack))))
  (Variables|Default|SetdistanceAlongSpline _distance))

(event EventTick
  (params (DeltaSeconds :type Float%20%28single-precision%29))
  (bind _returnvalue (Game|GetPlayerController 0))
  (bind _returnvalue_2 (Pawn|GetControlledPawn _returnvalue))
  (Utilities|IsValid (Variables|Default|GetcamTarget)
    (:Is%20Valid
      (Variables|Default|SetX%20Direction%20Player (.x (Transformation|GetActorForwardVector _returnvalue_2)))
      (CallFunction|GetCameraRotation (Variables|Default|GetX%20Direction%20Player) (Transformation|GetVelocity _returnvalue_2))
      (Transformation|SetWorldTransform (Variables|Default|GetsplineTarget) (Math|Transform|MakeTransform (Transformation|GetActorLocation _returnvalue_2) (Variables|Default|GetCamera%20Rotation) "1.000000,1.000000,1.000000") false false))))

(fn ConstructionScript)

(fn DegreesBetweenVectors
  (params (Vector1 :type Vector) (Vector2 :type Vector))
  (bind _returnvalue (Math|Vector|Normalize Vector2))
  (bind _returnvalue_2 (Math|Vector|Normalize Vector1))
  (bind _returnvalue_3 (Math|Conversions|ToVector2D(Vector) _returnvalue_2))
  (bind _returnvalue_4 (Math|Conversions|ToVector2D(Vector) _returnvalue))
  (bind _returnvalue_5 (* (.x _returnvalue_3) (.y _returnvalue_4)))
  (bind _returnvalue_6 (* (.y _returnvalue_3) (.x _returnvalue_4)))
  (bind _returnvalue_7 (* (.x _returnvalue_3) (.x _returnvalue_4)))
  (bind _returnvalue_8 (* (.y _returnvalue_3) (.y _returnvalue_4)))
  (bind _returnvalue_9 (- _returnvalue_5 _returnvalue_6))
  (bind _returnvalue_10 (+ _returnvalue_7 _returnvalue_8))
  (bind _returnvalue_11 (Class|KismetMathLibrary|DegAtan2 _returnvalue_10 _returnvalue_9))
  (bind _returnvalue_12 (+ _returnvalue_11 -9e+01))
  (if (< _returnvalue_12 -1.8e+02)
    (return (+ _returnvalue_12 3.6e+02))
    (elif (> _returnvalue_12 1.8e+02)
      (return (- _returnvalue_12 3.6e+02))
      (else
        (return _returnvalue_12)))))

(fn GetLocationsDistanceAlongSpline
  (params (givenLocation :type Vector) (givenSpline :type Spline%20Component%20Object%20Reference))
  (bind _returnvalue (Class|SplineComponent|FindInputKeyClosesttoWorldLocation givenSpline givenLocation))
  (bind _returnvalue_2 (Math|Float|Truncate _returnvalue))
  (bind _returnvalue_3 (Spline|GetDistanceAlongSplineatSplinePoint givenSpline _returnvalue_2))
  (return (+ _returnvalue_3 (* (- (Spline|GetDistanceAlongSplineatSplinePoint givenSpline (Math|Float|Truncate (+ _returnvalue 1.0))) _returnvalue_3) (- _returnvalue _returnvalue_2)))))

(fn GetCameraRotation
  (params (Player%20X%20Direction :type Float%20%28double-precision%29) (Player%20Velocity :type Vector))
  (if (Utilities|Operators|EqualEqual :A Player%20Velocity :ErrorTolerance 0.1)
    (if (> Player%20X%20Direction 0.75)
      (Variables|Default|SetCamera%20Rotation "0.000000,-70.000000,0.000000")
      (elif (< Player%20X%20Direction -0.75)
        (Variables|Default|SetCamera%20Rotation "0.000000,-110.000000,0.000000")))
    (else
      (Variables|Default|SetCamera%20Rotation "0.000000,-90.000000,0.000000"))))