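; BP_BreakableBox is a breakable box that can drop a coin when destroyed, with a random roll tagging item holders as SenseContainer.
; Overlaps from hero hitbox components request damage by message, and SendHitboxDamage lowers Health and updates the text display.
; When an overlap finds Health depleted, the box spawns a BP_MasterField for its geometry collection, whose collision damage is disabled, drops any coin and expires after a delay.
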(event OnComponentBeginOverlap(Box)
  (params (OverlappedComponent :type Primitive%20Component%20Object%20Reference) (OtherActor :type Actor%20Object%20Reference) (OtherComp :type Primitive%20Component%20Object%20Reference) (OtherBodyIndex :type Integer) (bFromSweep :type Boolean) (SweepResult :type Hit%20Result%20Structure%20%28by%20ref%29))
  (if (Components|ComponentHasTag OtherComp (Variables|Default|GetHeroHitbox%20Tag))
    (Class|BIGetHitboxDamage|GetHitboxDamage(Message) OtherActor self)
    (if (not (> (Variables|Default|GetHealth) 0.0))
      (CallFunction|Break)
      (Variables|Default|SetBroken true))))

(event Custom|Break
  (if (not (Variables|Default|GetBroken))
    (Utilities|FlowControl|Sequence
      (:then_0
        (Game|SpawnActorfromClass "/Game/_Interactions/BP_MasterField.BP_MasterField_C" (Math|Transform|MakeTransform (Transformation|GetActorLocation) "0, 0, 0" "1.000000,1.000000,1.000000") "AlwaysSpawn" "MultiplyWithRoot" 0 0)
        (if (Variables|Default|GethasItem)
          (Game|SpawnActorfromClass "/Game/_Interactions/Collectibles/BP_CollectibleCoin.BP_CollectibleCoin_C" (Math|Transform|MakeTransform (Transformation|GetActorLocation) "0, 0, 0" "1.000000,1.000000,1.000000") "AlwaysSpawn" "MultiplyWithRoot" 0 0)))
      (:then_1
        (CallFunction|Disappear)))))

(event Custom|Disappear
  (Actor|SetLifeSpan (Variables|Default|GetDisapearDelay)))

(event EventSendHitboxDamage
  (params (HitboxDamage :type Float%20%28double-precision%29))
  (Variables|Default|SetHealth (- (Variables|Default|GetHealth) HitboxDamage))
  (Rendering|Components|TextRender|SetText (Variables|Default|GetTextRender) (Utilities|Text|ToText(Float) (Variables|Default|GetHealth) "HalfToEven")))

(event EventBeginPlay
  (Rendering|Components|TextRender|SetText (Variables|Default|GetTextRender) (Utilities|Text|ToText(Float) (Variables|Default|GetHealth) "HalfToEven"))
  (Class|GeometryCollectionComponent|SetEnableDamagefromCollision (Variables|Default|GetBP_BreakableBox_GeometryCollection) false)
  (if (Math|Random|RandomBoolwithWeight 0.85)
    (Variables|Default|SethasItem true)
    (Utilities|Array|Add (Variables|Actor|GetTags) "SenseContainer")
    (Variables|Default|SetTags (Variables|Actor|GetTags))))

(fn ConstructionScript)