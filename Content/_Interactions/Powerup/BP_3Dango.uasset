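; BP_3Dango is an interaction actor in the powerup folder that presents a price prompt for a three-dango item.
; Any actor overlap adds the WB_3DangoPrice widget to the viewport and sets game-only input.
; When DidIBuy is false, it also shows the mouse cursor, plays Kyosuke's "sorry" voice line and opens his talk widget.
; DidIBuy is only read here, and no purchase or powerup effect happens in this graph.
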(event EventBeginPlay)

(event Collision|EventActorBeginOverlap
  (params (OtherActor :type Actor%20Object%20Reference))
  (bind _returnvalue (Game|GetPlayerController 0))
  (bind _returnvalue_2 (UserInterface|CreateWidget "/Game/_UI/Prices/WB_3DangoPrice.WB_3DangoPrice_C"))
  (UserInterface|Viewport|AddtoViewport _returnvalue_2 0)
  (Variables|/Script/Engine.PlayerController|SetbShowMouseCursor _returnvalue false)
  (if (Variables|Default|GetDidIBuy?)
    (Input|SetInputModeGameOnly _returnvalue false)
    (Variables|/Script/Engine.PlayerController|SetbShowMouseCursor _returnvalue false)
    (else
      (Input|SetInputModeGameOnly _returnvalue false)
      (Variables|/Script/Engine.PlayerController|SetbShowMouseCursor _returnvalue true)
      (Utilities|FlowControl|Sequence
        (:then_0
          (Audio|PlaySound2D "/Game/Sound/Voicelines/kyosukevoice_sorry.kyosukevoice_sorry" 1.0 1.0 0.0 0 0)
          (bind _returnvalue_3 (UserInterface|CreateWidget "/Game/_UI/TextBoxAssets/WB_TB_KyosukeTalk2.WB_TB_KyosukeTalk2_C"))
          (UserInterface|Viewport|AddtoViewport _returnvalue_3 0))))))

(event EventTick
  (params (DeltaSeconds :type Float%20%28single-precision%29)))

(event Input|ActionEvents|InputActionBuy
  (params (Key :type Key%20Structure :default "None")))

(fn ConstructionScript)