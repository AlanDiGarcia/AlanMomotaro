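; A breakable barrel that takes hits from the hero and can drop a collectible coin when destroyed.
; Overlaps from HeroHitBox-tagged components message the attacker for damage, which returns through SendHitboxDamage to lower Health and update a debug text.
; At the death cutoff, Break usually spawns a coin, spawns a short-lived FS_MasterField field actor, and sets the barrel to expire shortly after.
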(event OnComponentBeginOverlap(Capsule)
  (params (OverlappedComponent :type Primitive%20Component%20Object%20Reference) (OtherActor :type Actor%20Object%20Reference) (OtherComp :type Primitive%20Component%20Object%20Reference) (OtherBodyIndex :type Integer) (bFromSweep :type Boolean) (SweepResult :type Hit%20Result%20Structure%20%28by%20ref%29))
  (if (Components|ComponentHasTag OtherComp (Variables|Default|GetHeroHitBox))
    (Class|BIGetHitboxDamage|GetHitboxDamage(Message) OtherActor self)))

(event Custom|Break
  (if (Math|Random|RandomBoolwithWeight 0.25)
    _
    (else
      (Game|SpawnActorfromClass "/Game/_Interactions/BP_CollectibleCoin.BP_CollectibleCoin_C" (Math|Transform|MakeTransform (Transformation|GetActorLocation) "0, 0, 0" "1.000000,1.000000,1.000000") "AlwaysSpawn" "MultiplyWithRoot" 0 0)))
  (bind _returnvalue (Game|SpawnActorfromClass "/Engine/EditorResources/FieldNodes/FS_MasterField.FS_MasterField_C" (Math|Transform|MakeTransform (Transformation|GetActorLocation) "0, 0, 0" "1.000000,1.000000,1.000000") "Undefined" "MultiplyWithRoot" 0 0))
  (Actor|SetLifeSpan _returnvalue 1.0)
  (Actor|SetLifeSpan 4.0))

(event EventSendHitboxDamage
  (params (HitboxDamage :type Float%20%28double-precision%29))
  (Variables|Default|SetHealth (- (Variables|Default|GetHealth) HitboxDamage))
  (Rendering|Components|TextRender|SetText (Variables|Default|GetHealthDebug) (Utilities|Text|ToText(Float) (* (Variables|Default|GetHealth) 1e+02) "HalfToEven"))
  (if (not (> (Variables|Default|GetHealth) (Variables|Default|GetDeathCutoff)))
    (CallFunction|Break)))

(event EventBeginPlay
  (Rendering|Components|TextRender|SetText (Variables|Default|GetHealthDebug) (Utilities|Text|ToText(Float) (* (Variables|Default|GetHealth) 1e+02) "HalfToEven")))

(fn ConstructionScript)