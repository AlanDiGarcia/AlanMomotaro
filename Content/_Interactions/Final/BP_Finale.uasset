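; BP_Finale plays the game's scripted ending conversation between Akandoji, Momotaro, Kaori, Haruto and Satoshi.
; BeginPlay runs one linear chain of Delays, each beat pairing a 2D voice clip with a dedicated text widget added to the viewport.
; Momotaro, Kaori, Haruto and Satoshi meshes switch between talk and idle animations around their lines.
; The sequence closes by adding an audio component and showing the WB_TheEnd screen.
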(event EventBeginPlay
  (Audio|PlaySound2D "/Game/Sound/Voicelines/akandojivoice_scoff2.akandojivoice_scoff2" 1.0 1.0 0.0 0 0)
  (bind _returnvalue (UserInterface|CreateWidget "/Game/_UI/TextBoxAssets/Scene5/WB_TB_FinaleAkandoji1.WB_TB_FinaleAkandoji1_C"))
  (UserInterface|Viewport|AddtoViewport _returnvalue 0)
  (Utilities|FlowControl|Delay 2.0)
  (Components|Animation|PlayAnimation (Variables|Default|GetMomoMesh) "/Game/Characters/Momotaro/Animations/momotaroanimtalk.momotaroanimtalk" true)
  (Audio|PlaySound2D "/Game/Sound/Voicelines/momovoice_mmhmm.momovoice_mmhmm" 1.0 1.0 0.0 0 0)
  (bind _returnvalue_2 (UserInterface|CreateWidget "/Game/_UI/TextBoxAssets/Scene5/WB_TB_FinaleMomotaro1.WB_TB_FinaleMomotaro1_C"))
  (UserInterface|Viewport|AddtoViewport _returnvalue_2 0)
  (Utilities|FlowControl|Delay 3.0)
  (Components|Animation|PlayAnimation (Variables|Default|GetMomoMesh) "/Game/Characters/Momotaro/Animations/momotaroidle.momotaroidle" true)
  (Audio|PlaySound2D "/Game/Sound/Voicelines/akandojivoice_bwaaa.akandojivoice_bwaaa" 1.0 1.0 0.0 0 0)
  (bind _returnvalue_3 (UserInterface|CreateWidget "/Game/_UI/TextBoxAssets/Scene5/WB_TB_FinaleAkandoji2.WB_TB_FinaleAkandoji2_C"))
  (UserInterface|Viewport|AddtoViewport _returnvalue_3 0)
  (Utilities|FlowControl|Delay 2.0)
  (Components|Animation|PlayAnimation (Variables|Default|GetMomoMesh) "/Game/Characters/Momotaro/Animations/momotaroanimtalk.momotaroanimtalk" true)
  (Audio|PlaySound2D "/Game/Sound/Voicelines/momovoice_kiai.momovoice_kiai" 1.0 1.0 0.0 0 0)
  (bind _returnvalue_4 (UserInterface|CreateWidget "/Game/_UI/TextBoxAssets/Scene5/WB_TB_FinaleMomotaro2.WB_TB_FinaleMomotaro2_C"))
  (UserInterface|Viewport|AddtoViewport _returnvalue_4 0)
  (Utilities|FlowControl|Delay 3.0)
  (Components|Animation|PlayAnimation (Variables|Default|GetMomoMesh) "/Game/Characters/Momotaro/Animations/momotaroidle.momotaroidle" true)
  (Audio|PlaySound2D "/Game/Sound/Voicelines/akandojivoice_pain2.akandojivoice_pain2" 1.0 1.0 0.0 0 0)
  (bind _returnvalue_5 (UserInterface|CreateWidget "/Game/_UI/TextBoxAssets/Scene5/WB_TB_FinaleAkandoji3.WB_TB_FinaleAkandoji3_C"))
  (UserInterface|Viewport|AddtoViewport _returnvalue_5 0)
  (Utilities|FlowControl|Delay 4.0)
  (Audio|PlaySound2D "/Game/Sound/Voicelines/momovoice_YEAH.momovoice_YEAH" 1.0 1.0 0.0 0 0)
  (bind _returnvalue_6 (UserInterface|CreateWidget "/Game/_UI/TextBoxAssets/Scene5/WB_TB_FinaleEveryone.WB_TB_FinaleEveryone_C"))
  (UserInterface|Viewport|AddtoViewport _returnvalue_6 0)
  (Utilities|FlowControl|Delay 0.1)
  (Audio|PlaySound2D "/Game/Sound/Voicelines/kaorivoice_woohoo.kaorivoice_woohoo" 1.0 1.0 0.0 0 0)
  (Utilities|FlowControl|Delay 0.2)
  (Audio|PlaySound2D "/Game/Sound/Voicelines/harutovoice_phew.harutovoice_phew" 1.0 1.0 0.0 0 0)
  (Utilities|FlowControl|Delay 0.2)
  (Audio|PlaySound2D "/Game/Sound/Voicelines/satoshivoice_asexpected.satoshivoice_asexpected" 1.0 1.0 0.0 0 0)
  (Utilities|FlowControl|Delay 3.0)
  (Components|Animation|PlayAnimation (Variables|Default|GetKaoriMesh) "/Game/Characters/Kaori/Animations/kaorianimtalk.kaorianimtalk" true)
  (Audio|PlaySound2D "/Game/Sound/Voicelines/kaorivoice_hey.kaorivoice_hey" 1.0 1.0 0.0 0 0)
  (bind _returnvalue_7 (UserInterface|CreateWidget "/Game/_UI/TextBoxAssets/Scene5/WB_TB_FinaleKaori1.WB_TB_FinaleKaori1_C"))
  (UserInterface|Viewport|AddtoViewport _returnvalue_7 0)
  (Utilities|FlowControl|Delay 3.0)
  (Components|Animation|PlayAnimation (Variables|Default|GetKaoriMesh) "/Game/Characters/Kaori/Animations/kaoriidle.kaoriidle" true)
  (Components|Animation|PlayAnimation (Variables|Default|GetHarutoMesh) "/Game/Characters/Haruto/Animations/harutoanimtalk.harutoanimtalk" true)
  (Audio|PlaySound2D "/Game/Sound/Voicelines/harutovoice_yeahbut.harutovoice_yeahbut" 1.0 1.0 0.0 0 0)
  (bind _returnvalue_8 (UserInterface|CreateWidget "/Game/_UI/TextBoxAssets/Scene5/WB_TB_FinaleHaruto1.WB_TB_FinaleHaruto1_C"))
  (UserInterface|Viewport|AddtoViewport _returnvalue_8 0)
  (Utilities|FlowControl|Delay 3.0)
  (Components|Animation|SetAnimation (Variables|Default|GetHarutoMesh) "/Game/Characters/Haruto/Animations/harutoidle.harutoidle")
  (Components|Animation|SetAnimation (Variables|Default|GetSatoshiMesh) "/Game/Characters/Satoshi/Animations/satoshianimtalk.satoshianimtalk")
  (Audio|PlaySound2D "/Game/Sound/Voicelines/satoshivoice_hmm.satoshivoice_hmm" 1.0 1.0 0.0 0 0)
  (bind _returnvalue_9 (UserInterface|CreateWidget "/Game/_UI/TextBoxAssets/Scene5/WB_TB_FinaleSatoshi1.WB_TB_FinaleSatoshi1_C"))
  (UserInterface|Viewport|AddtoViewport _returnvalue_9 0)
  (Utilities|FlowControl|Delay 3.0)
  (Components|Animation|SetAnimation (Variables|Default|GetSatoshiMesh) "/Game/Characters/Satoshi/Animations/satoshianimidle.satoshianimidle")
  (Components|Animation|SetAnimation (Variables|Default|GetMomoMesh) "/Game/Characters/Momotaro/Animations/momotaroanimtalk.momotaroanimtalk")
  (Audio|PlaySound2D "/Game/Sound/Voicelines/momovoice_here.momovoice_here" 1.0 1.0 0.0 0 0)
  (bind _returnvalue_10 (UserInterface|CreateWidget "/Game/_UI/TextBoxAssets/Scene5/WB_TB_FinaleMomotaro3.WB_TB_FinaleMomotaro3_C"))
  (UserInterface|Viewport|AddtoViewport _returnvalue_10 0)
  (Utilities|FlowControl|Delay 3.0)
  (Components|Animation|PlayAnimation (Variables|Default|GetMomoMesh) "/Game/Characters/Momotaro/Animations/momotaroidle.momotaroidle" true)
  (Utilities|FlowControl|Delay 3.0)
  (Components|Animation|PlayAnimation (Variables|Default|GetMomoMesh) "/Game/Characters/Momotaro/Animations/momotaroanimtalk.momotaroanimtalk" true)
  (Audio|PlaySound2D "/Game/Sound/Voicelines/momovoice_takethat.momovoice_takethat" 1.0 1.0 0.0 0 0)
  (bind _returnvalue_11 (UserInterface|CreateWidget "/Game/_UI/TextBoxAssets/Scene5/WB_TB_FinaleMomotaro4.WB_TB_FinaleMomotaro4_C"))
  (UserInterface|Viewport|AddtoViewport _returnvalue_11 0)
  (Utilities|FlowControl|Delay 5.0)
  (Components|Animation|PlayAnimation (Variables|Default|GetMomoMesh) "/Game/Characters/Momotaro/Animations/momotaroidle.momotaroidle" true)
  (Audio|PlaySound2D "/Game/Sound/Voicelines/akandojivoice_nani.akandojivoice_nani" 1.0 1.0 0.0 0 0)
  (bind _returnvalue_12 (UserInterface|CreateWidget "/Game/_UI/TextBoxAssets/Scene5/WB_TB_FinaleAkandoji4.WB_TB_FinaleAkandoji4_C"))
  (UserInterface|Viewport|AddtoViewport _returnvalue_12 0)
  (Utilities|FlowControl|Delay 2.0)
  (AddComponent|AddAudioComponent false)
  (bind _returnvalue_13 (UserInterface|CreateWidget "/Game/_UI/WB_TheEnd.WB_TheEnd_C"))
  (UserInterface|Viewport|AddtoViewport _returnvalue_13 0))

(event Collision|EventActorBeginOverlap
  (params (OtherActor :type Actor%20Object%20Reference)))

(event EventTick
  (params (DeltaSeconds :type Float%20%28single-precision%29)))

(fn ConstructionScript)