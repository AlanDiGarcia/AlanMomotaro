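; Checkpoint actor that sets the hero's respawn point and shows a tutorial tip through two separate trigger boxes.
; Box fires once for a Hero-tagged actor, ignoring HeroHitbox components, sending its own location via SetRespawnPointMessage, then playing a voice cue and printing confirmation.
; Box1 adds a new WB_Tips6 widget to the viewport on every overlap by BP_PlayerMomotaro.
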(event OnComponentBeginOverlap(Box)
  (params (OverlappedComponent :type Primitive%20Component%20Object%20Reference) (OtherActor :type Actor%20Object%20Reference) (OtherComp :type Primitive%20Component%20Object%20Reference) (OtherBodyIndex :type Integer) (bFromSweep :type Boolean) (SweepResult :type Hit%20Result%20Structure%20%28by%20ref%29))
  (if (Actor|ActorHasTag OtherActor "Hero")
    (if (not (Components|ComponentHasTag OtherComp "HeroHitbox"))
      (Utilities|FlowControl|DoOnce false
        (:Completed
          (Class|BPISetRespawnPoint|SetRespawnPoint(Message) OtherActor (Transformation|GetActorLocation))
          (Audio|PlaySound2D "/Game/Sound/Voicelines/momovoice_YEAH.momovoice_YEAH" 1.0 1.0 0.0 0 0)
          (Development|PrintString "Checkpoint Set!"))))))

(event OnComponentBeginOverlap(Box1)
  (params (OverlappedComponent :type Primitive%20Component%20Object%20Reference) (OtherActor :type Actor%20Object%20Reference) (OtherComp :type Primitive%20Component%20Object%20Reference) (OtherBodyIndex :type Integer) (bFromSweep :type Boolean) (SweepResult :type Hit%20Result%20Structure%20%28by%20ref%29))
  (Utilities|Casting|CastToBP_PlayerMomotaro OtherActor)
  (bind _returnvalue (UserInterface|CreateWidget "/Game/_UI/Tips/WB_Tips6.WB_Tips6_C"))
  (UserInterface|Viewport|AddtoViewport _returnvalue 0))

(fn ConstructionScript)