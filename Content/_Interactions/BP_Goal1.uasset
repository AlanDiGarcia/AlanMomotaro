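; BP_Goal1 is a level goal trigger that completes the level when the hero reaches it.
; Its Box overlap accepts actors tagged Hero, ignoring components tagged HeroHitbox.
; It then prints a completion message, plays a sound at world origin, shows the LevelCompleteF widget and destroys Camera.
; An audio volume adjustment on the actor found by GetActorOfClass is left unconnected.
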(event OnComponentBeginOverlap(Box)
  (params (OverlappedComponent :type Primitive%20Component%20Object%20Reference) (OtherActor :type Actor%20Object%20Reference) (OtherComp :type Primitive%20Component%20Object%20Reference) (OtherBodyIndex :type Integer) (bFromSweep :type Boolean) (SweepResult :type Hit%20Result%20Structure%20%28by%20ref%29))
  (if (Actor|ActorHasTag OtherActor "Hero")
    (if (not (Components|ComponentHasTag OtherComp "HeroHitbox"))
      (Development|PrintString "Level Complete!" true true "(R=0.000000,G=0.587500,B=0.131716,A=1.000000)" 9.0 "complete")
      (bind _returnvalue (Actor|GetActorOfClass (Variables|Default|GetNewVar_0)))
      (Audio|PlaySoundatLocation "/Game/Sound/Music/BLAP-levelcomplete.BLAP-levelcomplete" "0, 0, 0" "0, 0, 0" 1.0 1.0 0.0 0 0 0 0)
      (bind _returnvalue_2 (UserInterface|CreateWidget "/Game/_UI/LevelCompleteF.LevelCompleteF_C"))
      (UserInterface|Viewport|AddtoViewport _returnvalue_2 0)
      (Actor|DestroyActor (Variables|Default|Getcamera)))))

(fn ConstructionScript)