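; BP_LockedGate is a gate that destroys itself once every actor referenced in its Keys array is no longer valid.
; A looping half-second timer counts the still-valid keys to update KeysRemaining.
; Tick writes that count to a text render and rotates it toward the camera component of the BP_Camera actor found at BeginPlay.
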(event Custom|CheckForComplete
  (bind _keys (Variables|Default|GetKeys))
  (Variables|Default|SetanyKeysRemaining false)
  (Variables|Default|SetcountKeys 0)
  (for (_ _array_index) _keys
    (Utilities|IsValid (Utilities|Array|Get(acopy) _keys _array_index)
      (:Is%20Valid
        (Variables|Default|SetanyKeysRemaining true)
        (Math|Integer|IncrementInt (Variables|Default|GetcountKeys)))))
  (if (Variables|Default|GetanyKeysRemaining)
    (Variables|Default|SetkeysRemaining (Variables|Default|GetcountKeys))
    (else
      (Variables|Default|SetkeysRemaining 0)
      (Actor|DestroyActor))))

(event EventTick
  (params (DeltaSeconds :type Float%20%28single-precision%29))
  (Rendering|Components|TextRender|SetText (Variables|Default|GetTextRender) (Utilities|Text|ToText(String) (Utilities|String|Append (Utilities|String|ToString(Integer) (Variables|Default|GetkeysRemaining)) " Key(s) Remaining")))
  (Transformation|SetWorldRotation (Variables|Default|GetTextRender) (Math|Rotator|FindLookatRotation (Transformation|GetActorLocation) (Transformation|GetWorldLocation (Variables|Default|GetCam))) false false))

(event EventBeginPlay
  (Utilities|Time|SetTimerbyEvent (delegate Custom|CheckForComplete) 0.5 true)
  (Rendering|Components|TextRender|SetText (Variables|Default|GetTextRender) (Utilities|Text|ToText(String) (Utilities|String|Append (Utilities|String|ToString(Integer) (Utilities|Array|Length (Variables|Default|GetKeys))) " Key(s) Remaining")))
  (bind _returnvalue (Actor|GetActorOfClass "/Game/Camera/BP_Camera.BP_Camera_C"))
  (Variables|Default|SetCam (Variables|/Game/Camera/BP_Camera.BP_Camera_C|GetCamera _returnvalue)))

(fn ConstructionScript)