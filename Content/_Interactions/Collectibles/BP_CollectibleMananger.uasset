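; Collectible manager that tallies the coins and gems picked up in the level.
; On BeginPlay it counts all BP_CollectibleGem actors to get the gem total.
; SendData routes a tag to the gem or coin counter, with unmatched tags counting as coins, and each increment prints progress on screen, gems labelled "Jade" against the total.
; An unconnected one-second delay loop that prints a number never runs.
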(event Custom|Add%20Coin
  (bind _coin_amount (Variables|Default|GetCoin%20Amount))
  (Math|Integer|IncrementInt _coin_amount
    (:%20%20
      (Development|PrintString (Utilities|String|Append "Coins: " (Utilities|String|ToString(Integer) _coin_amount)) true true "(R=0.000000,G=0.660000,B=1.000000,A=1.000000)" 6.0))))

(event Custom|Add%20Gem
  (Math|Integer|IncrementInt (Variables|Default|GetGem%20Amount)
    (:%20%20
      (Development|PrintString (Utilities|String|Append "Jade: " (Utilities|String|ToString(Integer) (Variables|Default|GetGem%20Amount)) "/" (Utilities|String|ToString(Integer) (Variables|Default|GetGem%20Count))) true true "(R=0.000000,G=0.660000,B=1.000000,A=1.000000)" 6.0))))

(event Custom|Count%20Gems
  (bind _outactors (Actor|GetAllActorsOfClass "/Game/_Interactions/Collectibles/BP_CollectibleGem.BP_CollectibleGem_C"))
  (Variables|Default|SetGem%20Count (Utilities|Array|Length _outactors)))

(event EventBeginPlay
  (CallFunction|CountGems))

(event EventSendData
  (params (Tag :type Name :default "None"))
  (switch name Tag
    (:Default
      (CallFunction|AddCoin :!label _label))
    (:Coin
      (goto _label))
    (:Gem
      (CallFunction|AddGem))))

(fn ConstructionScript)