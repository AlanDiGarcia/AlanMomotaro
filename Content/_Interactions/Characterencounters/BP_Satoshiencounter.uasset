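; Scripted encounter where Momotaro meets Satoshi, who joins the party after a dialogue with Momotaro and Kaori.
; Momotaro overlapping the Box trigger destroys it, then one hardcoded Delay chain drives chomp sounds, Satoshi's turn, his walk/talk/idle animation swaps, voice clips and a separate text-box widget per line.
; The chain ends by setting HasSatoshi on PC_ThirdPerson, showing the party-member notification and destroying the actor.
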(event OnComponentBeginOverlap(Box)
  (params (OverlappedComponent :type Primitive%20Component%20Object%20Reference) (OtherActor :type Actor%20Object%20Reference) (OtherComp :type Primitive%20Component%20Object%20Reference) (OtherBodyIndex :type Integer) (bFromSweep :type Boolean) (SweepResult :type Hit%20Result%20Structure%20%28by%20ref%29))
  (Utilities|Casting|CastToBP_PlayerMomotaro OtherActor)
  (Audio|PlaySound2D "/Game/Sound/Voicelines/momovoice_relief.momovoice_relief" 4.0 1.0 0.0 0 0)
  (bind _returnvalue (UserInterface|CreateWidget "/Game/_UI/TextBoxAssets/Scene2/WB_TB_MomotaroSEncounter1.WB_TB_MomotaroSEncounter1_C"))
  (UserInterface|Viewport|AddtoViewport _returnvalue 0)
  (Components|DestroyComponent (Variables|Character|GetBox))
  (Utilities|FlowControl|Delay 4.0)
  (Audio|PlaySound2D "/Game/Sound/SFX/chomp.chomp" 1.0 1.0 0.0 0 0)
  (Utilities|FlowControl|Delay 1.0)
  (Audio|PlaySound2D "/Game/Sound/SFX/chomp.chomp" 1.0 1.0 0.0 0 0)
  (Utilities|FlowControl|Delay 0.75)
  (Audio|PlaySound2D "/Game/Sound/SFX/chomp.chomp" 1.0 1.0 0.0 0 0)
  (Utilities|FlowControl|Delay 0.25)
  (Components|Animation|PlayAnimation (Variables|Character|GetMesh) "/Game/Characters/Satoshi/Animations/satoshianimwalk.satoshianimwalk" true)
  (Components|MoveComponentTo (Variables|Character|GetMesh) "0, 0, 0" "0.000000,90.000000,0.000000" false false 2.0 false)
  (Components|Animation|PlayAnimation (Variables|Character|GetMesh) "/Game/Characters/Satoshi/Animations/satoshianimtalk.satoshianimtalk" true)
  (Audio|PlaySound2D "/Game/Sound/Voicelines/satoshivoice_hello.satoshivoice_hello" 1.0 1.0 0.0 0 0)
  (bind _returnvalue_2 (UserInterface|CreateWidget "/Game/_UI/TextBoxAssets/Scene2/WB_TB_SatoshiTalkEncounter1.WB_TB_SatoshiTalkEncounter1_C"))
  (UserInterface|Viewport|AddtoViewport _returnvalue_2 0)
  (Utilities|FlowControl|Delay 4.0)
  (Components|Animation|PlayAnimation (Variables|Character|GetMesh) "/Game/Characters/Satoshi/Animations/satoshianimidle.satoshianimidle" true)
  (Audio|PlaySound2D "/Game/Sound/Voicelines/kaorivoice_huh.kaorivoice_huh" 1.0 1.0 0.0 0 0)
  (bind _returnvalue_3 (UserInterface|CreateWidget "/Game/_UI/TextBoxAssets/Scene2/WB_TB_KaoriSEncounter1.WB_TB_KaoriSEncounter1_C"))
  (UserInterface|Viewport|AddtoViewport _returnvalue_3 0)
  (Utilities|FlowControl|Delay 3.0)
  (Audio|PlaySound2D "/Game/Sound/Voicelines/momovoice_huh.momovoice_huh" 1.0 1.0 0.0 0 0)
  (bind _returnvalue_4 (UserInterface|CreateWidget "/Game/_UI/TextBoxAssets/Scene2/WB_TB_MomotaroSEncounter2.WB_TB_MomotaroSEncounter2_C"))
  (UserInterface|Viewport|AddtoViewport _returnvalue_4 0)
  (Utilities|FlowControl|Delay 3.0)
  (Components|Animation|PlayAnimation (Variables|Character|GetMesh) "/Game/Characters/Satoshi/Animations/satoshianimtalk.satoshianimtalk" true)
  (Audio|PlaySound2D "/Game/Sound/Voicelines/satoshivoice_chuckle.satoshivoice_chuckle" 1.0 1.0 0.0 0 0)
  (bind _returnvalue_5 (UserInterface|CreateWidget "/Game/_UI/TextBoxAssets/Scene2/WB_TB_SatoshiTalkEncounter2.WB_TB_SatoshiTalkEncounter2_C"))
  (UserInterface|Viewport|AddtoViewport _returnvalue_5 0)
  (Utilities|FlowControl|Delay 4.0)
  (Components|Animation|PlayAnimation (Variables|Character|GetMesh) "/Game/Characters/Satoshi/Animations/satoshianimidle.satoshianimidle" true)
  (Audio|PlaySound2D "/Game/Sound/Voicelines/momovoice_huh.momovoice_huh" 1.0 1.0 0.0 0 0)
  (bind _returnvalue_6 (UserInterface|CreateWidget "/Game/_UI/TextBoxAssets/Scene2/WB_TB_MomotaroSEncounter3.WB_TB_MomotaroSEncounter3_C"))
  (UserInterface|Viewport|AddtoViewport _returnvalue_6 0)
  (Utilities|FlowControl|Delay 4.0)
  (Components|Animation|PlayAnimation (Variables|Character|GetMesh) "/Game/Characters/Satoshi/Animations/satoshianimtalk.satoshianimtalk" true)
  (Audio|PlaySound2D "/Game/Sound/Voicelines/satoshivoice_sigh.satoshivoice_sigh" 1.0 1.0 0.0 0 0)
  (bind _returnvalue_7 (UserInterface|CreateWidget "/Game/_UI/TextBoxAssets/Scene2/WB_TB_SatoshiTalkEncounter3.WB_TB_SatoshiTalkEncounter3_C"))
  (UserInterface|Viewport|AddtoViewport _returnvalue_7 0)
  (Utilities|FlowControl|Delay 7.0)
  (Components|Animation|PlayAnimation (Variables|Character|GetMesh) "/Game/Characters/Satoshi/Animations/satoshianimidle.satoshianimidle" true)
  (Audio|PlaySound2D "/Game/Sound/Voicelines/momovoice_wantsome.momovoice_wantsome" 1.0 1.0 0.0 0 0)
  (bind _returnvalue_8 (UserInterface|CreateWidget "/Game/_UI/TextBoxAssets/Scene2/WB_TB_MomotaroSEncounter4.WB_TB_MomotaroSEncounter4_C"))
  (UserInterface|Viewport|AddtoViewport _returnvalue_8 0)
  (Utilities|FlowControl|Delay 4.0)
  (Audio|PlaySound2D "/Game/Sound/Voicelines/kaorivoice_comeon.kaorivoice_comeon" 1.0 1.0 0.0 0 0)
  (bind _returnvalue_9 (UserInterface|CreateWidget "/Game/_UI/TextBoxAssets/Scene2/WB_TB_KaoriSEncounter2.WB_TB_KaoriSEncounter2_C"))
  (UserInterface|Viewport|AddtoViewport _returnvalue_9 0)
  (Utilities|FlowControl|Delay 4.0)
  (Audio|PlaySound2D "/Game/Sound/Voicelines/momovoice_chill.momovoice_chill" 1.0 1.0 0.0 0 0)
  (bind _returnvalue_10 (UserInterface|CreateWidget "/Game/_UI/TextBoxAssets/Scene3/WB_TB_MomotaroHEncounter5.WB_TB_MomotaroHEncounter5_C"))
  (UserInterface|Viewport|AddtoViewport _returnvalue_10 0)
  (Utilities|FlowControl|Delay 4.0)
  (Audio|PlaySound2D "/Game/Sound/SFX/chomp.chomp" 1.0 1.0 0.0 0 0)
  (Utilities|FlowControl|Delay 3.0)
  (Components|Animation|PlayAnimation (Variables|Character|GetMesh) "/Game/Characters/Satoshi/Animations/satoshianimtalk.satoshianimtalk" true)
  (Audio|PlaySound2D "/Game/Sound/Voicelines/satoshivoice_hmm.satoshivoice_hmm" 1.0 1.0 0.0 0 0)
  (bind _returnvalue_11 (UserInterface|CreateWidget "/Game/_UI/TextBoxAssets/Scene2/WB_TB_SatoshiTalkEncounter4.WB_TB_SatoshiTalkEncounter4_C"))
  (UserInterface|Viewport|AddtoViewport _returnvalue_11 0)
  (Utilities|FlowControl|Delay 4.0)
  (Components|Animation|PlayAnimation (Variables|Character|GetMesh) "/Game/Characters/Satoshi/Animations/satoshianimidle.satoshianimidle" true)
  (Audio|PlaySound2D "/Game/Sound/Voicelines/kaorivoice_comeon.kaorivoice_comeon" 1.0 1.0 0.0 0 0)
  (bind _returnvalue_12 (UserInterface|CreateWidget "/Game/_UI/TextBoxAssets/Scene2/WB_TB_KaoriSEncounter3.WB_TB_KaoriSEncounter3_C"))
  (UserInterface|Viewport|AddtoViewport _returnvalue_12 0)
  (Utilities|FlowControl|Delay 4.0)
  (Components|Animation|PlayAnimation (Variables|Character|GetMesh) "/Game/Characters/Satoshi/Animations/satoshianimtalk.satoshianimtalk" true)
  (Audio|PlaySound2D "/Game/Sound/Voicelines/satoshivoice_meh.satoshivoice_meh" 1.0 1.0 0.0 0 0)
  (bind _returnvalue_13 (UserInterface|CreateWidget "/Game/_UI/TextBoxAssets/Scene2/WB_TB_SatoshiTalkEncounter5.WB_TB_SatoshiTalkEncounter5_C"))
  (UserInterface|Viewport|AddtoViewport _returnvalue_13 0)
  (Utilities|FlowControl|Delay 4.0)
  (Components|Animation|PlayAnimation (Variables|Character|GetMesh) "/Game/Characters/Satoshi/Animations/satoshianimidle.satoshianimidle" true)
  (Audio|PlaySound2D "/Game/Sound/Voicelines/kaorivoice_grr.kaorivoice_grr" 1.0 1.0 0.0 0 0)
  (bind _returnvalue_14 (UserInterface|CreateWidget "/Game/_UI/TextBoxAssets/Scene2/WB_TB_KaoriSEncounter4.WB_TB_KaoriSEncounter4_C"))
  (UserInterface|Viewport|AddtoViewport _returnvalue_14 0)
  (Utilities|FlowControl|Delay 4.0)
  (Components|Animation|PlayAnimation (Variables|Character|GetMesh) "/Game/Characters/Satoshi/Animations/satoshianimtalk.satoshianimtalk" true)
  (Audio|PlaySound2D "/Game/Sound/Voicelines/satoshivoice_hmm.satoshivoice_hmm" 1.0 1.0 0.0 0 0)
  (bind _returnvalue_15 (UserInterface|CreateWidget "/Game/_UI/TextBoxAssets/Scene2/WB_TB_SatoshiTalkEncounter6.WB_TB_SatoshiTalkEncounter6_C"))
  (UserInterface|Viewport|AddtoViewport _returnvalue_15 0)
  (Utilities|FlowControl|Delay 7.0)
  (Components|Animation|PlayAnimation (Variables|Character|GetMesh) "/Game/Characters/Satoshi/Animations/satoshianimidle.satoshianimidle" true)
  (Audio|PlaySound2D "/Game/Sound/Voicelines/kaorivoice_hey.kaorivoice_hey" 1.0 1.0 0.0 0 0)
  (bind _returnvalue_16 (UserInterface|CreateWidget "/Game/_UI/TextBoxAssets/Scene2/WB_TB_KaoriSEncounter5.WB_TB_KaoriSEncounter5_C"))
  (UserInterface|Viewport|AddtoViewport _returnvalue_16 0)
  (Utilities|FlowControl|Delay 3.0)
  (Audio|PlaySound2D "/Game/Sound/Voicelines/momovoice_mmhmm.momovoice_mmhmm" 1.0 1.0 0.0 0 0)
  (bind _returnvalue_17 (UserInterface|CreateWidget "/Game/_UI/TextBoxAssets/Scene2/WB_TB_MomotaroSEncounter6.WB_TB_MomotaroSEncounter6_C"))
  (UserInterface|Viewport|AddtoViewport _returnvalue_17 0)
  (Utilities|FlowControl|Delay 4.0)
  (Components|Animation|PlayAnimation (Variables|Character|GetMesh) "/Game/Characters/Satoshi/Animations/satoshianimtalk.satoshianimtalk" true)
  (Audio|PlaySound2D "/Game/Sound/Voicelines/satoshivoice_chuckle.satoshivoice_chuckle" 1.0 1.0 0.0 0 0)
  (bind _returnvalue_18 (UserInterface|CreateWidget "/Game/_UI/TextBoxAssets/Scene2/WB_TB_SatoshiTalkEncounter8.WB_TB_SatoshiTalkEncounter8_C"))
  (UserInterface|Viewport|AddtoViewport _returnvalue_18 0)
  (Utilities|FlowControl|Delay 4.0)
  (Components|Animation|PlayAnimation (Variables|Character|GetMesh) "/Game/Characters/Satoshi/Animations/satoshianimidle.satoshianimidle" true)
  (Audio|PlaySound2D "/Game/Sound/Voicelines/momovoice_cmon.momovoice_cmon" 1.0 1.0 0.0 0 0)
  (bind _returnvalue_19 (UserInterface|CreateWidget "/Game/_UI/TextBoxAssets/Scene2/WB_TB_MomotaroSEncounter7.WB_TB_MomotaroSEncounter7_C"))
  (UserInterface|Viewport|AddtoViewport _returnvalue_19 0)
  (Utilities|FlowControl|Delay 3.0)
  (bind _aspc_third_person (Utilities|Casting|CastToPC_ThirdPerson (Game|GetPlayerController 0)))
  (Variables|/Game/_Core/PC_ThirdPerson.PC_ThirdPerson_C|SetHasSatoshi _aspc_third_person true)
  (Audio|PlaySound2D "/Game/Sound/SFX/partymemberget.partymemberget" 1.0 1.0 0.0 0 0)
  (bind _returnvalue_20 (UserInterface|CreateWidget "/Game/_UI/Tips/WB_PlayerAddedSatoshi.WB_PlayerAddedSatoshi_C"))
  (UserInterface|Viewport|AddtoViewport _returnvalue_20 0)
  (Actor|DestroyActor))

(fn ConstructionScript)