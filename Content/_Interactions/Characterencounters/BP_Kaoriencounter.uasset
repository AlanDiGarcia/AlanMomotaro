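; Scripted story encounter where Kaori joins Momotaro's party, triggered when BP_PlayerMomotaro overlaps its Box.
; One linear Delay-timed chain walks Kaori's mesh over, then alternates talk and idle animations, voice sounds and a new dialogue widget per line.
; It ends by setting KaoriInParty after a PC_ThirdPerson cast.
; The party-added fanfare, widget and DestroyActor are disconnected, and nothing guards against retriggering.
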(event OnComponentBeginOverlap(Box)
  (params (OverlappedComponent :type Primitive%20Component%20Object%20Reference) (OtherActor :type Actor%20Object%20Reference) (OtherComp :type Primitive%20Component%20Object%20Reference) (OtherBodyIndex :type Integer) (bFromSweep :type Boolean) (SweepResult :type Hit%20Result%20Structure%20%28by%20ref%29))
  (bind _mesh (Variables|Character|GetMesh))
  (bind _mesh_2 (Variables|Character|GetMesh))
  (bind _asbp_player_momotaro (Utilities|Casting|CastToBP_PlayerMomotaro OtherActor))
  (Components|Animation|PlayAnimation (Variables|Character|GetMesh) "/Game/Characters/Kaori/Animations/kaorianimtalk.kaorianimtalk" true)
  (Audio|PlaySound2D 0 1.0 1.0 0.0 0 0)
  (bind _returnvalue (UserInterface|CreateWidget "/Game/_UI/TextBoxAssets/Scene1/WB_TB_KaoriTalkEncounter.WB_TB_KaoriTalkEncounter_C"))
  (UserInterface|Viewport|AddtoViewport _returnvalue 0)
  (Utilities|FlowControl|Delay 2.0)
  (Components|Animation|SetAnimation _mesh_2 "/Game/Characters/Kaori/Animations/kaorianimwalk.kaorianimwalk")
  (Components|MoveComponentTo _mesh_2 "-120.000000,0.000000,0.000000" "0.000000,90.000000,0.000000" false false 0.2 false)
  (Components|Animation|PlayAnimation _mesh "/Game/Characters/Kaori/Animations/kaorianimtalk.kaorianimtalk" true)
  (Audio|PlaySound2D 0 1.0 1.0 0.0 0 0)
  (bind _returnvalue_2 (UserInterface|CreateWidget "/Game/_UI/TextBoxAssets/Scene1/WB_TB_KaoriTalkEncounter1.WB_TB_KaoriTalkEncounter1_C"))
  (UserInterface|Viewport|AddtoViewport _returnvalue_2 0)
  (Utilities|FlowControl|Delay 4.0)
  (Components|Animation|PlayAnimation (Variables|Character|GetMesh) "/Game/Characters/Kaori/Animations/kaoriidle.kaoriidle" true)
  (Audio|PlaySound2D "/Game/Sound/Voicelines/momovoice_YEAH.momovoice_YEAH" 1.0 1.0 0.0 0 0)
  (bind _returnvalue_3 (UserInterface|CreateWidget "/Game/_UI/TextBoxAssets/Scene1/WB_TB_MomotaroKEncounter1.WB_TB_MomotaroKEncounter1_C"))
  (UserInterface|Viewport|AddtoViewport _returnvalue_3 0)
  (Utilities|FlowControl|Delay 4.0)
  (Components|Animation|PlayAnimation _mesh "/Game/Characters/Kaori/Animations/kaorianimtalk.kaorianimtalk" true)
  (Audio|PlaySound2D 0 1.0 1.0 0.0 0 0)
  (bind _returnvalue_4 (UserInterface|CreateWidget "/Game/_UI/TextBoxAssets/Scene1/WB_TB_KaoriTalkEncounter2.WB_TB_KaoriTalkEncounter2_C"))
  (UserInterface|Viewport|AddtoViewport _returnvalue_4 0)
  (Utilities|FlowControl|Delay 4.0)
  (Components|Animation|PlayAnimation (Variables|Character|GetMesh) "/Game/Characters/Kaori/Animations/kaoriidle.kaoriidle" true)
  (Audio|PlaySound2D "/Game/Sound/Voicelines/momovoice_wantsome.momovoice_wantsome" 1.0 1.0 0.0 0 0)
  (bind _returnvalue_5 (UserInterface|CreateWidget "/Game/_UI/TextBoxAssets/Scene1/WB_TB_MomotaroKEncounter2.WB_TB_MomotaroKEncounter2_C"))
  (UserInterface|Viewport|AddtoViewport _returnvalue_5 0)
  (Utilities|FlowControl|Delay 4.0)
  (Components|Animation|PlayAnimation (Variables|Character|GetMesh) "/Game/Characters/Kaori/Animations/kaorianimtalk.kaorianimtalk" true)
  (Audio|PlaySound2D 0 1.0 1.0 0.0 0 0)
  (bind _returnvalue_6 (UserInterface|CreateWidget "/Game/_UI/TextBoxAssets/Scene1/WB_TB_KaoriTalkEncounter3.WB_TB_KaoriTalkEncounter3_C"))
  (UserInterface|Viewport|AddtoViewport _returnvalue_6 0)
  (Utilities|FlowControl|Delay 4.0)
  (Components|Animation|PlayAnimation (Variables|Character|GetMesh) "/Game/Characters/Kaori/Animations/kaoriidle.kaoriidle" true)
  (Audio|PlaySound2D "/Game/Sound/Voicelines/momovoice_here.momovoice_here" 1.0 1.0 0.0 0 0)
  (bind _returnvalue_7 (UserInterface|CreateWidget "/Game/_UI/TextBoxAssets/Scene1/WB_TB_MomotaroKEncounter3.WB_TB_MomotaroKEncounter3_C"))
  (UserInterface|Viewport|AddtoViewport _returnvalue_7 0)
  (Utilities|FlowControl|Delay 3.0)
  (Audio|PlaySound2D "/Game/Sound/SFX/chomp.chomp" 1.0 1.0 0.0 0 0)
  (Utilities|FlowControl|Delay 0.2)
  (Components|Animation|PlayAnimation (Variables|Character|GetMesh) "/Game/Characters/Kaori/Animations/kaorianimtalk.kaorianimtalk" true)
  (Audio|PlaySound2D 0 1.0 1.0 0.0 0 0)
  (bind _returnvalue_8 (UserInterface|CreateWidget "/Game/_UI/TextBoxAssets/Scene1/WB_TB_KaoriTalkEncounter4.WB_TB_KaoriTalkEncounter4_C"))
  (UserInterface|Viewport|AddtoViewport _returnvalue_8 0)
  (Utilities|FlowControl|Delay 4.0)
  (Components|Animation|PlayAnimation (Variables|Character|GetMesh) "/Game/Characters/Kaori/Animations/kaoriidle.kaoriidle" true)
  (Audio|PlaySound2D "/Game/Sound/Voicelines/momovoice_hey.momovoice_hey" 1.0 1.0 0.0 0 0)
  (bind _returnvalue_9 (UserInterface|CreateWidget "/Game/_UI/TextBoxAssets/Scene1/WB_TB_MomotaroKEncounter4.WB_TB_MomotaroKEncounter4_C"))
  (UserInterface|Viewport|AddtoViewport _returnvalue_9 0)
  (Utilities|FlowControl|Delay 4.0)
  (Components|Animation|PlayAnimation (Variables|Character|GetMesh) "/Game/Characters/Kaori/Animations/kaorianimtalk.kaorianimtalk" true)
  (Audio|PlaySound2D 0 1.0 1.0 0.0 0 0)
  (bind _returnvalue_10 (UserInterface|CreateWidget "/Game/_UI/TextBoxAssets/Scene1/WB_TB_KaoriTalkEncounter5.WB_TB_KaoriTalkEncounter5_C"))
  (UserInterface|Viewport|AddtoViewport _returnvalue_10 0)
  (Utilities|FlowControl|Delay 4.0)
  (Components|Animation|PlayAnimation (Variables|Character|GetMesh) "/Game/Characters/Kaori/Animations/kaoriidle.kaoriidle" true)
  (Audio|PlaySound2D "/Game/Sound/Voicelines/momovoice_mmhmm.momovoice_mmhmm" 1.0 1.0 0.0 0 0)
  (bind _returnvalue_11 (UserInterface|CreateWidget "/Game/_UI/TextBoxAssets/Scene1/WB_TB_MomotaroKEncounter5.WB_TB_MomotaroKEncounter5_C"))
  (UserInterface|Viewport|AddtoViewport _returnvalue_11 0)
  (Utilities|FlowControl|Delay 4.0)
  (Components|Animation|PlayAnimation (Variables|Character|GetMesh) "/Game/Characters/Kaori/Animations/kaorianimtalk.kaorianimtalk" true)
  (Audio|PlaySound2D 0 1.0 1.0 0.0 0 0)
  (bind _returnvalue_12 (UserInterface|CreateWidget "/Game/_UI/TextBoxAssets/Scene1/WB_TB_KaoriTalkEncounter6.WB_TB_KaoriTalkEncounter6_C"))
  (UserInterface|Viewport|AddtoViewport _returnvalue_12 0)
  (Utilities|FlowControl|Delay 4.0)
  (Components|Animation|PlayAnimation (Variables|Character|GetMesh) "/Game/Characters/Kaori/Animations/kaoriidle.kaoriidle" true)
  (Audio|PlaySound2D "/Game/Sound/Voicelines/momovoice_mmhmm.momovoice_mmhmm" 1.0 1.0 0.0 0 0)
  (bind _returnvalue_13 (UserInterface|CreateWidget "/Game/_UI/TextBoxAssets/Scene1/WB_TB_KaoriTalkEncounter6.WB_TB_KaoriTalkEncounter6_C"))
  (UserInterface|Viewport|AddtoViewport _returnvalue_13 0)
  (Utilities|FlowControl|Delay 4.0)
  (Components|Animation|PlayAnimation (Variables|Character|GetMesh) "/Game/Characters/Kaori/Animations/kaorianimtalk.kaorianimtalk" true)
  (Audio|PlaySound2D 0 1.0 1.0 0.0 0 0)
  (bind _returnvalue_14 (UserInterface|CreateWidget "/Game/_UI/TextBoxAssets/Scene1/WB_TB_KaoriTalkEncounter7.WB_TB_KaoriTalkEncounter7_C"))
  (UserInterface|Viewport|AddtoViewport _returnvalue_14 0)
  (Utilities|FlowControl|Delay 4.0)
  (Components|Animation|PlayAnimation (Variables|Character|GetMesh) "/Game/Characters/Kaori/Animations/kaoriidle.kaoriidle" true)
  (Audio|PlaySound2D "/Game/Sound/Voicelines/momovoice_cmon.momovoice_cmon" 1.0 1.0 0.0 0 0)
  (bind _returnvalue_15 (UserInterface|CreateWidget "/Game/_UI/TextBoxAssets/Scene1/WB_TB_MomotaroKEncounter7.WB_TB_MomotaroKEncounter7_C"))
  (UserInterface|Viewport|AddtoViewport _returnvalue_15 0)
  (Utilities|FlowControl|Delay 4.0)
  (Utilities|Casting|CastToPC_ThirdPerson (Game|GetPlayerController 0))
  (Variables|Default|SetKaoriInParty true))

(event EventBeginPlay)

(event Collision|EventActorBeginOverlap
  (params (OtherActor :type Actor%20Object%20Reference)))

(event EventTick
  (params (DeltaSeconds :type Float%20%28single-precision%29)))

(fn ConstructionScript)