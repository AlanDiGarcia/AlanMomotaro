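; Scripted encounter actor for Haruto that plays a one-time dialogue scene when Momotaro enters its trigger box.
; The overlap destroys the box, then runs a timed chain of voice lines, text-box widgets, mesh animations and MoveComponentTo steps.
; The chain stops after Momotaro's third voice cue; the last exchange and the party-recruit ending that sets HasHaruto and destroys the actor are unconnected.
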(event OnComponentBeginOverlap(Box)
  (params (OverlappedComponent :type Primitive%20Component%20Object%20Reference) (OtherActor :type Actor%20Object%20Reference) (OtherComp :type Primitive%20Component%20Object%20Reference) (OtherBodyIndex :type Integer) (bFromSweep :type Boolean) (SweepResult :type Hit%20Result%20Structure%20%28by%20ref%29))
  (Utilities|Casting|CastToBP_PlayerMomotaro OtherActor)
  (Audio|PlaySound2D "/Game/Sound/Voicelines/momovoice_hey.momovoice_hey" 4.0 1.0 0.0 0 0)
  (bind _returnvalue (UserInterface|CreateWidget "/Game/_UI/TextBoxAssets/Scene3/WB_TB_MomotaroHEncounter1.WB_TB_MomotaroHEncounter1_C"))
  (UserInterface|Viewport|AddtoViewport _returnvalue 0)
  (Components|DestroyComponent (Variables|Character|GetBox))
  (Utilities|FlowControl|Delay 4.0)
  (Audio|PlaySound2D "/Game/Sound/Voicelines/harutovoice_fear.harutovoice_fear" 1.0 1.0 0.0 0 0)
  (bind _returnvalue_2 (UserInterface|CreateWidget "/Game/_UI/TextBoxAssets/Scene3/WB_TB_HarutoTalkEncounter1.WB_TB_HarutoTalkEncounter1_C"))
  (UserInterface|Viewport|AddtoViewport _returnvalue_2 0)
  (Components|Animation|PlayAnimation (Variables|Character|GetMesh) "/Game/Characters/Haruto/Animations/harutoanimwalk.harutoanimwalk" true)
  (Components|MoveComponentTo (Variables|Character|GetMesh) "300.000000,0.000000,0.000000" "0.000000,-90.000000,0.000000" false false 0.5 false)
  (Audio|PlaySound2D "/Game/Sound/Voicelines/momovoice_huh.momovoice_huh" 1.0 1.0 0.0 0 0)
  (bind _returnvalue_3 (UserInterface|CreateWidget "/Game/_UI/TextBoxAssets/Scene3/WB_TB_MomotaroHEncounter2.WB_TB_MomotaroHEncounter2_C"))
  (UserInterface|Viewport|AddtoViewport _returnvalue_3 0)
  (Utilities|FlowControl|Delay 4.0)
  (Components|MoveComponentTo (Variables|Character|GetMesh) "100.000000,0.000000,0.000000" "0.000000,90.000000,0.000000" false false 0.5 false)
  (Components|Animation|PlayAnimation (Variables|Character|GetMesh) "/Game/Characters/Haruto/Animations/harutoanimtalk.harutoanimtalk" true)
  (Audio|PlaySound2D "/Game/Sound/Voicelines/harutovoice_wat.harutovoice_wat" 1.0 1.0 0.0 0 0)
  (bind _returnvalue_4 (UserInterface|CreateWidget "/Game/_UI/TextBoxAssets/Scene3/WB_TB_HarutoTalkEncounter2.WB_TB_HarutoTalkEncounter2_C"))
  (UserInterface|Viewport|AddtoViewport _returnvalue_4 0)
  (Utilities|FlowControl|Delay 4.0)
  (Components|Animation|PlayAnimation (Variables|Character|GetMesh) "/Game/Characters/Haruto/Animations/harutoidle.harutoidle" true)
  (Audio|PlaySound2D "/Game/Sound/Voicelines/momovoice_hey.momovoice_hey" 1.0 1.0 0.0 0 0))

(fn ConstructionScript)