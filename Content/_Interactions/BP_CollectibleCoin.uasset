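; Collectible coin pickup that spins and is collected when the hero touches it.
; On BeginPlay, a timeline drives the Cube mesh's rotation, starting from a random time so coins do not spin in sync.
; When an actor tagged "Hero" overlaps the Box, it finds BP_CollectibleMananger with GetActorOfClass, calls AddCoin and destroys itself.
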(event OnComponentBeginOverlap(Box)
  (params (OverlappedComponent :type Primitive%20Component%20Object%20Reference) (OtherActor :type Actor%20Object%20Reference) (OtherComp :type Primitive%20Component%20Object%20Reference) (OtherBodyIndex :type Integer) (bFromSweep :type Boolean) (SweepResult :type Hit%20Result%20Structure%20%28by%20ref%29))
  (if (Actor|ActorHasTag OtherActor "Hero")
    (bind _returnvalue (Actor|GetActorOfClass "/Game/_Interactions/BP_CollectibleMananger.BP_CollectibleMananger_C"))
    (Default|AddCoin _returnvalue)
    (Actor|DestroyActor)))

(event Custom|Coin%20Spin
  (Utilities|FlowControl|Sequence
    (:then_0
      (bind _newtrack_0 (Timeline|Timeline%20Coin%20Spin SetNewTime)
        (:Update
          (Transformation|SetWorldRotation (Variables|Default|GetCube) (Math|Rotator|Lerp(Rotator) "0.000000,360.000000,0.000000" "0, 0, 0" _newtrack_0) false false))))
    (:then_1
      (Timeline|Timeline%20Coin%20Spin Play))))

(event EventBeginPlay
  (CallFunction|CoinSpin))

(fn ConstructionScript)