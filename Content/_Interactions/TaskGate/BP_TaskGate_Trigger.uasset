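; Trigger that turns on its linked task gates when the Hero enters, then releases them once an objective is met.
; The first overlap by a non-AI Hero stores the player and start time, enables the gates and starts a looping objective-check timer.
; Depending on the objective, the check waits until no Enemy-tagged actors remain near the player or the gate time elapses, then clears the timer and disables the gates.
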(event OnComponentBeginOverlap(Trigger)
  (params (OverlappedComponent :type Primitive%20Component%20Object%20Reference) (OtherActor :type Actor%20Object%20Reference) (OtherComp :type Primitive%20Component%20Object%20Reference) (OtherBodyIndex :type Integer) (bFromSweep :type Boolean) (SweepResult :type Hit%20Result%20Structure%20%28by%20ref%29))
  (if (and (Actor|ActorHasTag OtherActor "Hero") (not (Actor|ActorHasTag OtherActor "AI")))
    (Utilities|FlowControl|DoOnce false
      (:Completed
        (Variables|Default|SetPlayer OtherActor)
        (Variables|Time|SetTimeAtStart (Utilities|Time|GetGameTimeinSeconds))
        (for _array_element (Variables|Default|GetTaskGates)
          (Default|EnableGate _array_element))
        (bind _returnvalue (Utilities|Time|SetTimerbyEvent (delegate Custom|CheckObjectiveWin) 0.5 true))))))

(event Custom|CheckObjectiveWin
  (switch Utilities|FlowControl|Switch|SwitchonE_TaskGateObjectives (Variables|Default|GetObjective)
    (:NewEnumerator0
      (Variables|Default|SetisObjectiveNotComplete false)
      (bind _outactors (Actor|GetAllActorswithTag "Enemy"))
      (for _array_element _outactors
        (if (<= (Math|Vector|Distance(Vector) (Transformation|GetActorLocation _array_element) (Transformation|GetActorLocation (Variables|Default|GetPlayer))) (Variables|Default|GetEnemyKillDistanceCheck))
          (Variables|Default|SetisObjectiveNotComplete true)))
      (if (not (Variables|Default|GetisObjectiveNotComplete))
        (Utilities|Time|ClearandInvalidateTimerbyHandle (stale OnComponentBeginOverlap(Trigger) _returnvalue) :!label _label)
        (for _array_element_2 (Variables|Default|GetTaskGates)
          (Default|DisableGate _array_element_2))))
    (:NewEnumerator1
      (if (>= (- (Utilities|Time|GetGameTimeinSeconds) (Variables|Time|GetTimeAtStart)) (Variables|Time|GetgateTime))
        (goto _label)))))

(event EventUpdatePlayer
  (params (NewPlayerPawn :type Pawn%20Object%20Reference))
  (Variables|Default|SetPlayer NewPlayerPawn))

(fn ConstructionScript)